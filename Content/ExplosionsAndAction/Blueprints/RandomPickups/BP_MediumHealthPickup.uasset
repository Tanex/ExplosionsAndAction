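; Medium health pickup that restores a fixed amount of health to the character that collects it.
; Its HandlePickup event casts the actor to BP_BaseCharacter, adds to Health, plays the health powerup sound on it and caps Health at MaxHealth.
; The construction script only calls the parent's, and BeginPlay and overlap events are unused.
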(event `self.ReceiveBeginPlay`)

(event `self.ReceiveActorBeginOverlap`
  (params (OtherActor :type "Actor Object Reference")))

(event `self.HandlePickup`
  (params (Actor :type "Actor Object Reference"))
  (bind _asbp_base_character (cast `/Game/ExplosionsAndAction/Blueprints/Characters/BP_BaseCharacter` Actor))
  (bind _output_get (set `/Game/ExplosionsAndAction/Blueprints/Characters/BP_BaseCharacter.Health` (+ (`/Game/ExplosionsAndAction/Blueprints/Characters/BP_BaseCharacter.Health` _asbp_base_character) 20.0) _asbp_base_character))
  (`/Game/ExplosionsAndAction/Blueprints/Characters/BP_BaseCharacter.PlaySound` _asbp_base_character "/Game/ExplosionsAndAction/Sounds/Powerup_Health.Powerup_Health")
  (bind _maxhealth (`/Game/ExplosionsAndAction/Blueprints/Characters/BP_BaseCharacter.MaxHealth` _asbp_base_character))
  (if (> _output_get _maxhealth)
    (set `/Game/ExplosionsAndAction/Blueprints/Characters/BP_BaseCharacter.Health` _maxhealth _asbp_base_character)))

(fn `UserConstructionScript`
  (`parent.UserConstructionScript`))