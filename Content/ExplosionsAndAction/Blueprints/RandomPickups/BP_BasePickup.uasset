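; Base pickup actor that hides when a BP_BaseCharacter overlaps it and reappears after a respawn delay.
; The overlap hides the actor and disables the RenderComponent's overlap events on whichever machine detects it.
; Only the authority starts the Respawn timer, which restores both, and calls HandlePickup with the overlapping actor.
; HandlePickup is empty here, leaving the pickup effect to child Blueprints.
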(event `self.RenderComponent.OnComponentBeginOverlap`
  (params (OtherActor :type "Actor Object Reference") (OtherComp :type "PrimitiveComponent Object Reference") (OtherBodyIndex :type Integer) (bFromSweep :type Boolean) (SweepResult :type "EngineTypes.HitResult Structure (by ref)"))
  (cast `/Game/ExplosionsAndAction/Blueprints/Characters/BP_BaseCharacter` OtherActor)
  (`self.SetActorHiddenInGame` true)
  (set `PrimitiveComponent.bGenerateOverlapEvents` false (`self.RenderComponent`))
  (`/Engine/EditorBlueprintResources/ActorMacros.Switch Has Authority`
    (:`Authority`
      (`KismetSystemLibrary.K2_SetTimer` null "Respawn" (`self.RespawnTime`))
      (`self.HandlePickup` OtherActor))))

(event `Respawn`
  (`self.SetActorHiddenInGame` false)
  (set `PrimitiveComponent.bGenerateOverlapEvents` true (`self.RenderComponent`)))

(fn `HandlePickup`
  (params (Actor :type "Actor Object Reference")))

(fn `UserConstructionScript`)