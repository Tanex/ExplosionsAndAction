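; Mage's primary weapon, a child weapon Blueprint that overrides Shoot to cast an ammo actor at a mana cost.
; It fires only when the owning BP_MageCharacter is not flying, drawing mana from that character's JetpackFuel.
; The projectile spawns ahead of BarrelDirection, with the barrel's Y position zeroed, alongside a sound and a brief Casting flag.
; The construction script sets spawn distance and mana cost.
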(event `self.Shoot`
  (params (State :type Boolean) (Instigator :type "Pawn Object Reference"))
  (bind _barreldirection (`self.BarrelDirection`))
  ;[1 1 1] Overloaded Shoot function
  (if State
    (bind _asbp_mage_character (cast `/Game/ExplosionsAndAction/Blueprints/Characters/BP_MageCharacter` (`ActorComponent.GetOwner` (`SceneComponent.GetAttachParent` (`self.K2_GetRootComponent`)))))
    (if (`/Game/ExplosionsAndAction/Blueprints/Characters/BP_MageCharacter.Flying` _asbp_mage_character)
      _
      (elif (>= (`/Game/ExplosionsAndAction/Blueprints/Characters/BP_BaseCharacter.Jetpack Fuel` _asbp_mage_character) (`self.ManaCost`))
        (set `/Game/ExplosionsAndAction/Blueprints/Characters/BP_MageCharacter.Casting` true _asbp_mage_character)
        (set `/Game/ExplosionsAndAction/Blueprints/Characters/BP_BaseCharacter.Jetpack Fuel` (- (`/Game/ExplosionsAndAction/Blueprints/Characters/BP_BaseCharacter.Jetpack Fuel` _asbp_mage_character) (`self.ManaCost`)) _asbp_mage_character)
        (`|SpawnActorFromClass` (`self.Ammo`) (`KismetMathLibrary.MakeTransform` (+ (* (`SceneComponent.GetForwardVector` _barreldirection) (`self.BulletSpawnDistance`)) (* (.location (`SceneComponent.K2_GetComponentToWorld` _barreldirection)) (1.0 0.0 1.0))) (.rotation (`SceneComponent.K2_GetComponentToWorld` _barreldirection)) (.scale (`SceneComponent.K2_GetComponentToWorld` _barreldirection))) false Instigator)
        (`self.PlaySound` (`self.SoundEffect`))
        (`KismetSystemLibrary.Delay` 0.2)
        (set `/Game/ExplosionsAndAction/Blueprints/Characters/BP_MageCharacter.Casting` false _asbp_mage_character)))))

(fn `UserConstructionScript`
  (`parent.UserConstructionScript`)
  (set `self.BulletSpawnDistance` 50.0)
  (set `self.ManaCost` 30.0))