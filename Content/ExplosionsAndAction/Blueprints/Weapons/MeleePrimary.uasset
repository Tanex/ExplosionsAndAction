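; Melee primary weapon that plays a one-shot Paper2D flipbook and sound on Shoot and logs the attack to FFA player stats.
; Two capsule overlaps on the side the control yaw faces damage blocks first, then characters, with blockers' owners meant to be excluded from the second.
; Damage varies via the game mode's seeded random stream and doubles with the double-damage pickup; reloading does nothing.
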(event `PlayAttackAnimation`
  (`SceneComponent.SetVisibility` false)
  (`SceneComponent.SetVisibility` true)
  (`PaperFlipbookComponent.PlayFromStart` (`self.PaperFlipbook`)))

(event `self.Shoot`
  (params (State :type Boolean) (Instigator :type "Pawn Object Reference"))
  (bind _returnvalue (`self.K2_GetActorLocation` Instigator))
  (bind _returnvalue_2 (`Pawn.GetController` Instigator))
  (bind _array (`|MakeArray` Instigator :!type "Actor Object Reference"))
  (bind _damage (`self.Damage`))
  (bind _returnvalue_3 (select `bool` (< (.yaw (`Controller.GetControlRotation` _returnvalue_2)) 90.0) :`false` (+ _returnvalue (-68.0 0.0 0.0)) :`true` (+ _returnvalue (68.0 0.0 0.0))))
  (`self.LogWeaponFire`)
  (`self.PlayAttackAnimation`)
  (`self.PlaySound` (`self.SoundEffect`))
  (bind _asbp_base_character (cast `/Game/ExplosionsAndAction/Blueprints/Characters/BP_BaseCharacter` Instigator))
  (bind _asbase_game_mode (cast `/Game/ExplosionsAndAction/Blueprints/GameModes/BaseGameMode` (`GameplayStatics.GetGameMode`)))
  ;[1 1 1] Check if anyone is blocking
  (bind _outactors (`KismetSystemLibrary.CapsuleOverlapActors_NEW` _returnvalue_3 45.0 54.0 (`|MakeArray` "ObjectTypeQuery2" :!type "EngineTypes.EObjectTypeQuery Enum") "/Game/ExplosionsAndAction/Blueprints/Blocks/BP_BaseBlock.BP_BaseBlock_C"))
  (for _array_element _outactors
    (bind _asbp_base_block (cast `/Game/ExplosionsAndAction/Blueprints/Blocks/BP_BaseBlock` _array_element))
    (bind _returnvalue_4 (* (`KismetMathLibrary.RandomFloatInRangeFromStream` 0.9 1.1 (`/Game/ExplosionsAndAction/Blueprints/GameModes/BaseGameMode.RNG` _asbase_game_mode)) (select `bool` (`/Game/ExplosionsAndAction/Blueprints/Characters/PickupHandler.HasDoubleDamage` (`/Game/ExplosionsAndAction/Blueprints/Characters/BP_BaseCharacter.PickupHandler` _asbp_base_character)) :`false` _damage :`true` (* _damage 2.0))))
    (`GameplayStatics.ApplyDamage` _asbp_base_block _returnvalue_4 _returnvalue_2 self "/Script/Engine.DamageType")
    ;;[1 1 1] Ignore everyone who's block was hit
    (`KismetArrayLibrary.Array_AddUnique` _array (`ActorComponent.GetOwner` (`SceneComponent.GetAttachParent` (`self.K2_GetRootComponent` _asbp_base_block)))))
  ;[1 1 1] Damage Actors
  (bind _outactors_2 (`KismetSystemLibrary.CapsuleOverlapActors_NEW` _returnvalue_3 50.0 64.0 (`|MakeArray` "ObjectTypeQuery3" :!type "EngineTypes.EObjectTypeQuery Enum") "/Game/ExplosionsAndAction/Blueprints/Characters/BP_BaseCharacter.BP_BaseCharacter_C" _array))
  (for _array_element_2 _outactors_2
    (`GameplayStatics.ApplyDamage` _array_element_2 _returnvalue_4 _returnvalue_2 self "/Script/Engine.DamageType")))

(event `self.ReloadWeapon`
  (params (Instigator :type "Pawn Object Reference")))

(event `self.PaperFlipbook.OnFinishedPlaying`
  (`SceneComponent.SetVisibility` false)
  (`SceneComponent.SetVisibility` true))

(event `LogWeaponFire`
  (bind _asffaplayer_state (cast `/Game/ExplosionsAndAction/Blueprints/GameModes/FFAPlayerState` (`Controller.PlayerState` (`self.GetInstigatorController` (`ActorComponent.GetOwner` (`SceneComponent.GetAttachParent` (`self.K2_GetRootComponent`)))))))
  (`/Game/ExplosionsAndAction/Blueprints/GameModes/FFAPlayerState.UpdateWeaponStats` _asffaplayer_state 41 0 0 1 0))

(fn `UserConstructionScript`
  (`parent.UserConstructionScript`)
  (`PaperFlipbookComponent.SetLooping` (`self.PaperFlipbook`) false))