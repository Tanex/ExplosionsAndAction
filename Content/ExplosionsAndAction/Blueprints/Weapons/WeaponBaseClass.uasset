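; Base weapon Blueprint that handles firing, magazine ammo and timed reloading for a BP_BaseCharacter.
; Shoot runs through the TriggerDelay gate macro for held automatic fire with a cooldown, spawning the Ammo actor and muzzle flash at the barrel, with the barrel's Y position zeroed.
; ReloadWeapon counts down in a Delay loop, then refills from reserve ammo.
; The character receives ammo and reload updates and plays the weapon's sounds.
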(event `Shoot`
  (params (State :type Boolean :default false) (Instigator :type "Pawn Object Reference"))
  (bind _barreldirection (`self.BarrelDirection`))
  ;[1 1 1] Shoots the weapon
  (`self.TriggerDelay` State (`self.FireDelay`)
    (:`Triggered Function`
      (if (`self.Reloading`)
        _
        (elif (> (`self.AmmoInMagazine`) 0)
          (`|SpawnActorFromClass` (`self.Ammo`) (`KismetMathLibrary.MakeTransform` (+ (* (`SceneComponent.GetForwardVector` _barreldirection) (`self.BulletSpawnDistance`)) (* (.location (`SceneComponent.K2_GetComponentToWorld` _barreldirection)) (1.0 0.0 1.0))) (.rotation (`SceneComponent.K2_GetComponentToWorld` _barreldirection)) (.scale (`SceneComponent.K2_GetComponentToWorld` _barreldirection))) false Instigator)
          (`GameplayStatics.SpawnEmitterAttached` "/Game/ExplosionsAndAction/Particles/MuzzleFlash/MuzzleFlash.MuzzleFlash" (`self.BarrelDirection`) "None" (`KismetMathLibrary.MakeVector` (- (`self.BulletSpawnDistance`) 60.0)) (struct) "KeepRelativeOffset" false)
          (set `self.AmmoInMagazine` (- (`self.AmmoInMagazine`) 1))
          (bind _asbp_base_character (cast `/Game/ExplosionsAndAction/Blueprints/Characters/BP_BaseCharacter` Instigator))
          (`/Game/ExplosionsAndAction/Blueprints/Characters/BP_BaseCharacter.UpdateAmmoInMag` _asbp_base_character)
          (`self.PlaySound` "/Game/ExplosionsAndAction/Sounds/Soldier_Machine_Gun_Fire.Soldier_Machine_Gun_Fire"))))))

(event `ReloadWeapon`
  (params (Instigator :type "Pawn Object Reference"))
  ;[1 1 1] Reloads Weapon
  (if (< (`self.AmmoInMagazine`) (`self.MagazineSize`))
    (if (> (`self.AvailableAmmo`) 0)
      (if (not (`self.Reloading`))
        (`self.PlaySound` "/Game/ExplosionsAndAction/Sounds/Soldier_Machine_Gun_Reload_var2.Soldier_Machine_Gun_Reload_var2")
        (set `self.ReloadProgress` (`self.ReloadTime`))
        (set `self.Reloading` true)
        (if (> (`self.ReloadProgress`) 0.01) :!label _label
          (`KismetSystemLibrary.Delay` 0.1)
          (set `self.ReloadProgress` (- (`self.ReloadProgress`) 0.1))
          (bind _asbp_base_character (cast `/Game/ExplosionsAndAction/Blueprints/Characters/BP_BaseCharacter` Instigator))
          (`/Game/ExplosionsAndAction/Blueprints/Characters/BP_BaseCharacter.UpdateReloadProg` _asbp_base_character)
          (goto _label)
          (else
            (set `self.AvailableAmmo` (+ (`self.AmmoInMagazine`) (`self.AvailableAmmo`)))
            (if (>= (`self.AvailableAmmo`) (`self.MagazineSize`))
              (set `self.AmmoInMagazine` (`self.MagazineSize`))
              (set `self.AvailableAmmo` (- (`self.AvailableAmmo`) (`self.AmmoInMagazine`)))
              (else
                (set `self.AmmoInMagazine` (`self.AvailableAmmo`))
                (set `self.AvailableAmmo` 0)))
            (set `self.Reloading` false)
            (bind _asbp_base_character_2 (cast `/Game/ExplosionsAndAction/Blueprints/Characters/BP_BaseCharacter` Instigator))
            (`/Game/ExplosionsAndAction/Blueprints/Characters/BP_BaseCharacter.UpdateAmmoInMag` _asbp_base_character_2)
            (`self.PlaySound` "/Game/ExplosionsAndAction/Sounds/Soldier_Machine_Gun_Reload_var2.Soldier_Machine_Gun_Reload_var2")))))))

(fn `PlaySound`
  (params (Sound :type "SoundWave Object Reference"))
  (bind _asbp_base_character (cast `/Game/ExplosionsAndAction/Blueprints/Characters/BP_BaseCharacter` (`ActorComponent.GetOwner` (`SceneComponent.GetAttachParent` (`self.K2_GetRootComponent`)))))
  (`/Game/ExplosionsAndAction/Blueprints/Characters/BP_BaseCharacter.PlaySound` _asbp_base_character Sound))

(fn `UserConstructionScript`
  (set `self.Reloading` false))