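; Replicated pickup actor that gives an overlapping character a random powerup: double damage, health or ammo.
; The local player sees a pickup particle, while the authority destroys the actor, rolls a random enum entry and applies it with sound, message and player-state stats.
; Health and ammo are capped, though secondary ammo only refills when primary overflows.
; Taking damage pushes the pickup along the damage causer's velocity.
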(event `self.ReceiveAnyDamage`
  (params (Damage :type "Float (single-precision)") (DamageType :type "DamageType Object Reference") (InstigatedBy :type "Controller Object Reference") (DamageCauser :type "Actor Object Reference"))
  ;[1 1 1] Bullet Hit
  (`PrimitiveComponent.AddImpulse` (/ (* (`self.GetVelocity` DamageCauser) Damage) 50.0) "None" true))

(event `self.RenderComponent.OnComponentBeginOverlap`
  (params (OtherActor :type "Actor Object Reference") (OtherComp :type "PrimitiveComponent Object Reference") (OtherBodyIndex :type Integer) (bFromSweep :type Boolean) (SweepResult :type "EngineTypes.HitResult Structure (by ref)"))
  (bind _returnvalue (enumcount `/Game/ExplosionsAndAction/Blueprints/RandomPickups/RandomPickupEnum`))
  (bind _controlledcharacter (`self.ControlledCharacter`))
  (bind _controlledcharacter_2 (`self.ControlledCharacter`))
  (bind _controlledcharacter_3 (`self.ControlledCharacter`))
  (bind _controlledcharacter_4 (`self.ControlledCharacter`))
  ;[1 1 1] Player Hit
  (bind _asbp_base_character (cast `/Game/ExplosionsAndAction/Blueprints/Characters/BP_BaseCharacter` OtherActor))
  (if (`Controller.IsLocalPlayerController` (`self.GetInstigatorController` OtherActor))
    (`GameplayStatics.SpawnEmitterAtLocation` "/Game/ExplosionsAndAction/Particles/P_PickupEffect.P_PickupEffect" (`self.K2_GetActorLocation`)))
  (`/Engine/EditorBlueprintResources/ActorMacros.Switch Has Authority`
    (:`Authority`
      (`self.K2_DestroyActor`)
      (set `self.ControlledCharacter` _asbp_base_character)
      (if (> _returnvalue 0)
        (switch `/Game/ExplosionsAndAction/Blueprints/RandomPickups/RandomPickupEnum` (cast `/Game/ExplosionsAndAction/Blueprints/RandomPickups/RandomPickupEnum` (`KismetMathLibrary.Conv_IntToByte` (`KismetMathLibrary.RandomIntegerInRange` 0 (- _returnvalue 1))))
          (:`NewEnumerator0`
            (`/Game/ExplosionsAndAction/Blueprints/Characters/PickupHandler.SetDoubleDamage` _controlledcharacter)
            (`self.PlaySound` "/Game/ExplosionsAndAction/Sounds/Powerup_DoubleDamage.Powerup_DoubleDamage")
            (bind _asbase_player_controller (cast `/Game/ExplosionsAndAction/Blueprints/Controllers/BasePlayerController` (`Pawn.GetController` _controlledcharacter)))
            (`/Game/ExplosionsAndAction/Blueprints/Controllers/BasePlayerController.PrintMsg` _asbase_player_controller "Double Damage!")
            (bind _asffaplayer_state (cast `/Game/ExplosionsAndAction/Blueprints/GameModes/FFAPlayerState` (`Pawn.PlayerState` _controlledcharacter)))
            (`/Game/ExplosionsAndAction/Blueprints/GameModes/FFAPlayerState.UpdatePickupStats` _asffaplayer_state 1 1 0))
          (:`NewEnumerator1`
            (bind _output_get (set `/Game/ExplosionsAndAction/Blueprints/Characters/BP_BaseCharacter.Health` (+ (`/Game/ExplosionsAndAction/Blueprints/Characters/BP_BaseCharacter.Health` _controlledcharacter_2) 50.0) _controlledcharacter_2))
            (`self.PlaySound` "/Game/ExplosionsAndAction/Sounds/Powerup_Health.Powerup_Health")
            (bind _asbase_player_controller_2 (cast `/Game/ExplosionsAndAction/Blueprints/Controllers/BasePlayerController` (`Pawn.GetController` _controlledcharacter_3)))
            (`/Game/ExplosionsAndAction/Blueprints/Controllers/BasePlayerController.PrintMsg` _asbase_player_controller_2 "+50 Health")
            (bind _asffaplayer_state_2 (cast `/Game/ExplosionsAndAction/Blueprints/GameModes/FFAPlayerState` (`Pawn.PlayerState` _controlledcharacter_3)))
            (`/Game/ExplosionsAndAction/Blueprints/GameModes/FFAPlayerState.UpdatePickupStats` _asffaplayer_state_2 2 1 0)
            (if (> _output_get 150.0)
              (set `/Game/ExplosionsAndAction/Blueprints/Characters/BP_BaseCharacter.Health` 150.0 _controlledcharacter_3)))
          (:`NewEnumerator2`
            (`self.PlaySound` "/Game/ExplosionsAndAction/Sounds/Crate_Bounce_var1.Crate_Bounce_var1")
            (bind _asbase_player_controller_3 (cast `/Game/ExplosionsAndAction/Blueprints/Controllers/BasePlayerController` (`Pawn.GetController` _controlledcharacter_4)))
            (`/Game/ExplosionsAndAction/Blueprints/Controllers/BasePlayerController.PrintMsg` _asbase_player_controller_3 "+20% Ammo")
            (bind (_primaryweapon _secondaryweapon) (`/Game/ExplosionsAndAction/Blueprints/Characters/MacroLib.GetWeapons` _controlledcharacter_4)
              (:`Out`
                (bind _maxammo (`/Game/ExplosionsAndAction/Blueprints/Weapons/WeaponBaseClass.MaxAmmo` _primaryweapon))
                (bind _returnvalue_2 (/ (* _maxammo 20) 100))
                (if (< _returnvalue_2 1)
                  (set `/Game/ExplosionsAndAction/Blueprints/Weapons/WeaponBaseClass.AvailableAmmo` (+ (`/Game/ExplosionsAndAction/Blueprints/Weapons/WeaponBaseClass.AvailableAmmo` _primaryweapon) 1) _primaryweapon)
                  (else
                    (bind _availableammo (`/Game/ExplosionsAndAction/Blueprints/Weapons/WeaponBaseClass.AvailableAmmo` _primaryweapon))
                    (set `/Game/ExplosionsAndAction/Blueprints/Weapons/WeaponBaseClass.AvailableAmmo` (+ _returnvalue_2 _availableammo) _primaryweapon)))
                (if (> _availableammo _maxammo)
                  (set `/Game/ExplosionsAndAction/Blueprints/Weapons/WeaponBaseClass.AvailableAmmo` _maxammo _primaryweapon)
                  (bind _maxammo_2 (`/Game/ExplosionsAndAction/Blueprints/Weapons/WeaponBaseClass.MaxAmmo` _secondaryweapon))
                  (bind _returnvalue_3 (/ (* _maxammo_2 20) 100))
                  (if (< _returnvalue_3 1)
                    (set `/Game/ExplosionsAndAction/Blueprints/Weapons/WeaponBaseClass.AvailableAmmo` (+ (`/Game/ExplosionsAndAction/Blueprints/Weapons/WeaponBaseClass.AvailableAmmo` _secondaryweapon) 1) _secondaryweapon)
                    (else
                      (bind _availableammo_2 (`/Game/ExplosionsAndAction/Blueprints/Weapons/WeaponBaseClass.AvailableAmmo` _secondaryweapon))
                      (set `/Game/ExplosionsAndAction/Blueprints/Weapons/WeaponBaseClass.AvailableAmmo` (+ _returnvalue_3 _availableammo_2) _secondaryweapon)))
                  (if (> _availableammo_2 _maxammo_2)
                    (set `/Game/ExplosionsAndAction/Blueprints/Weapons/WeaponBaseClass.AvailableAmmo` _maxammo_2 _secondaryweapon)
                    (`/Game/ExplosionsAndAction/Blueprints/Characters/BP_BaseCharacter.UpdateAmmoInMag` _controlledcharacter_4)
                    (bind _asffaplayer_state_3 (cast `/Game/ExplosionsAndAction/Blueprints/GameModes/FFAPlayerState` (`Pawn.PlayerState` _controlledcharacter_4)))
                    (`/Game/ExplosionsAndAction/Blueprints/GameModes/FFAPlayerState.UpdatePickupStats` _asffaplayer_state_3 3 1 0)))))))))))

(event `PlaySound`
  (params (Sound :type "SoundWave Object Reference"))
  (`GameplayStatics.PlaySoundAtLocation` Sound))

(fn `UserConstructionScript`
  (`ActorComponent.SetIsReplicated` true))