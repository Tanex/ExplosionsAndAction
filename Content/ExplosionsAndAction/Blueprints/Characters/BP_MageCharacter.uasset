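; Mage player character: a flipbook-sprite child class that can switch from jumping to flight, re-armed whenever it can jump again.
; While flying, jump and block inputs move it up and down; otherwise they jump or trigger the child-actor block.
; Tick tints the sprite by active weapon and recharges mana, stored as jetpack fuel.
; Animation follows casting and movement state, and damage and deaths are logged to FFAPlayerState class stats.
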(event `self.ReceiveBeginPlay`
  (`parent.ReceiveBeginPlay`))

(event `self.RotateWeapon`
  (params (WeaponRotation :type "Object.Rotator Structure"))
  (`SceneComponent.K2_SetRelativeRotation` WeaponRotation)
  (`SceneComponent.K2_SetRelativeRotation` WeaponRotation)
  (`SceneComponent.K2_SetRelativeRotation` WeaponRotation))

(event `self.AnimationUpdate`
  ;[1 1 1] Update Animation Depending on Action
  (`PaperFlipbookComponent.SetFlipbook` (`self.Sprite`) (select `bool` (`self.Casting`) :`false` (select `bool` (`NavMovementComponent.IsMovingOnGround` (`self.CharacterMovement`)) :`false` (select `bool` (`self.Flying`) :`false` "/Game/ExplosionsAndAction/Sprites/MageClass/MageJump.MageJump" :`true` "/Game/ExplosionsAndAction/Sprites/MageClass/MageFly.MageFly" :!type "PaperFlipbook Object Reference") :`true` (select `bool` (> (`KismetMathLibrary.VSize` (`self.GetVelocity`)) 0.0) :`false` "/Game/ExplosionsAndAction/Sprites/MageClass/MageIdle.MageIdle" :`true` "/Game/ExplosionsAndAction/Sprites/MageClass/MageWalk.MageWalk" :!type "PaperFlipbook Object Reference")) :`true` "/Game/ExplosionsAndAction/Sprites/MageClass/MageAttack.MageAttack"))
  (`SceneComponent.SetWorldScale3D` (2.5 3.45 3.45)))

(event `self.ReceiveTick`
  (params (DeltaSeconds :type "Float (single-precision)"))
  (bind _sprite (`self.Sprite`))
  ;[1 1 1] Recharge Mana
  (if (== (`self.ActiveWeapon`) 1)
    (`PaperFlipbookComponent.SetSpriteColor` _sprite (struct :`R` 0.64 :`G` 0.64 :`B` 1.0 :`A` 1.0))
    (else
      (`PaperFlipbookComponent.SetSpriteColor` _sprite (struct :`R` 1.0 :`G` 0.366678 :`A` 1.0))))
  (`parent.ReceiveTick` DeltaSeconds)
  (if (`self.CanJump`)
    (set `self.CanFly` true))
  (if (< (`self.Jetpack Fuel`) (`self.Max Fuel`))
    (bind _output_get (set `self.Jetpack Fuel` (+ (* DeltaSeconds (`self.Fuel Recharge Rate`)) (`self.Jetpack Fuel`))))
    (if (> _output_get (`self.Max Fuel`))
      (set `self.Jetpack Fuel` (`self.Max Fuel`)))))

(event `self.EventStartFly`
  (params (MouseLocation :type "Object.Vector Structure"))
  ;[1 1 1] Set Movement Mode
  (if (`self.CanFly`)
    (set `self.Flying` true)
    (`CharacterMovementComponent.SetMovementMode` "MOVE_Flying")
    (set `self.CanFly` false)))

(event `self.EventStopFly`
  ;[1 1 1] Set Movement Mode
  (if (`self.Flying`)
    (set `self.Flying` false)
    (`CharacterMovementComponent.SetMovementMode` "MOVE_Walking")))

(event `self.MovementJump`
  (params (Axis :type "Float (single-precision)"))
  ;[1 1 1] Fly up if Flying, else Jump
  (if (`self.Flying`)
    (`self.AddMovementInput` (0.0 0.0 1.5) Axis)
    (elif (`self.JumpButtonPressed`)
      (`self.Jump`)
      (if (`self.CanJump`)
        _)
      (else
        (`self.StopJumping`)))))

(event `Fly Down`
  ;[1 1 1] Fly down if Flying, else Block
  (`self.AddMovementInput` (0.0 0.0 1.5) -1.0))

(event `self.BlockPressed`
  ;[1 1 1] Fly down if Flying, else Block
  (if (`self.Flying`)
    (`self.Fly Down` self)
    (else
      (bind _asbp_base_block (cast `/Game/ExplosionsAndAction/Blueprints/Blocks/BP_BaseBlock` (`ChildActorComponent.ChildActor` (`self.Block`))))
      (`/Game/ExplosionsAndAction/Blueprints/Blocks/BP_BaseBlock.BlockPressed` _asbp_base_block))))

(event `self.LogDeath2`
  (bind _asffaplayer_state (cast `/Game/ExplosionsAndAction/Blueprints/GameModes/FFAPlayerState` (`self.PlayerState`)))
  (`/Game/ExplosionsAndAction/Blueprints/GameModes/FFAPlayerState.UpdateClassStats` _asffaplayer_state 30 0 1))

(event `self.LogDamage2`
  (params (Damage :type "Float (single-precision)"))
  (bind _asffaplayer_state (cast `/Game/ExplosionsAndAction/Blueprints/GameModes/FFAPlayerState` (`self.PlayerState`)))
  (`/Game/ExplosionsAndAction/Blueprints/GameModes/FFAPlayerState.UpdateClassStats` _asffaplayer_state 30 (`KismetMathLibrary.FFloor` Damage) 0))

(fn `UserConstructionScript`
  (`parent.UserConstructionScript`)
  (`self.SetActorHiddenInGame` (`ChildActorComponent.ChildActor` (`self.PrimaryWeapon`)) true)
  (`self.SetActorHiddenInGame` (`ChildActorComponent.ChildActor` (`self.SecondaryWeapon`)) true)
  (`SceneComponent.SetRelativeScale3D` (2.5 3.45 3.45))
  (bind _output_get (set `self.Max Fuel` 100.0))
  (set `self.Jetpack Fuel` _output_get)
  (set `self.Fuel Recharge Rate` 15.0)
  (`PrimitiveComponent.SetLockedAxis` (`self.CapsuleComponent`) "Y")
  (`PrimitiveComponent.SetLockedAxis` (`self.Sprite`) "Y"))