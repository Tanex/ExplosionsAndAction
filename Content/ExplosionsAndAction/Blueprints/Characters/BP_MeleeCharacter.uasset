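; Melee class character for a sprite-based side-on game, with a cooldown-limited weapon swing and a grappling hook in place of flying.
; Fly input spawns and closes the hook from the secondary weapon's barrel, while weapon swap is stubbed out.
; Authority-side Tick shows the rope child actor, rotating and stretching it toward the hook or its target.
; It also picks movement flipbooks and logs damage and deaths to FFAPlayerState.
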(event `self.ChangeWeaponOffsetLeft`
  (`SceneComponent.K2_SetRelativeLocation` (0.0 -0.1 0.0))
  (`SceneComponent.K2_SetRelativeLocation` (0.0 0.1 0.0)))

(event `self.ChangeWeaponOffsetRight`
  (`SceneComponent.K2_SetRelativeLocation` (0.0 0.1 0.0))
  (`SceneComponent.K2_SetRelativeLocation` (0.0 -0.1 0.0)))

(event `self.RotateWeapon`
  (params (WeaponRotation :type "Object.Rotator Structure"))
  (`SceneComponent.K2_SetRelativeRotation` WeaponRotation))

(event `self.AnimationUpdate`
  (`PaperFlipbookComponent.SetFlipbook` (`self.Sprite`) (select `bool` (`NavMovementComponent.IsMovingOnGround` (`self.CharacterMovement`)) :`false` "/Game/ExplosionsAndAction/Sprites/MeleeCharacter/MeleeCharacter_Jumping_Flipbook.MeleeCharacter_Jumping_Flipbook" :`true` (select `bool` (> (`KismetMathLibrary.VSize` (`self.GetVelocity`)) 0.0) :`false` "/Game/ExplosionsAndAction/Sprites/MeleeCharacter/MeleeCharacter_Idle.MeleeCharacter_Idle" :`true` "/Game/ExplosionsAndAction/Sprites/MeleeCharacter/MeleeCharacter_Running.MeleeCharacter_Running" :!type "PaperFlipbook Object Reference")))
  (`SceneComponent.SetRelativeScale3D` (2.5 0.0 3.45)))

(event `self.EventStartFly`
  (params (MouseLocation :type "Object.Vector Structure"))
  (`self.FireGrapplingHook`))

(event `self.EventStopWeaponFire`
  ;[1 1 1] Functionality removal
)

(event `self.WeaponSwap`
  ;[1 1 1] Functionality removal
)

(event `self.EventStopFly`
  (`self.RemoveGrapplingHook`))

(event `FireGrapplingHook`
  ;[1 1 1] Spawn Grapplinghook
  (if (`self.CanFireGrappling`)
    (set `self.CanFireGrappling` false)
    (bind _asweapon_base_class (cast `/Game/ExplosionsAndAction/Blueprints/Weapons/WeaponBaseClass` (`ChildActorComponent.ChildActor` (`self.SecondaryWeapon`))))
    (bind _barreldirection (`/Game/ExplosionsAndAction/Blueprints/Weapons/WeaponBaseClass.BarrelDirection` _asweapon_base_class))
    (bind _returnvalue (`|SpawnActorFromClass` "/Game/ExplosionsAndAction/Blueprints/Characters/BP_GrapplingHook.BP_GrapplingHook_C" (`KismetMathLibrary.MakeTransform` (+ (* (`SceneComponent.GetForwardVector` _barreldirection) (`self.GrapplingHookSpawnDistance`)) (* (.location (`SceneComponent.K2_GetComponentToWorld` _barreldirection)) (1.0 0.0 1.0))) (.rotation (`SceneComponent.K2_GetComponentToWorld` _barreldirection)) (.scale (`SceneComponent.K2_GetComponentToWorld` _barreldirection))) false self))
    (set `self.GrapplingHook` _returnvalue)))

(event `RemoveGrapplingHook`
  ;[1 1 1] Remove the grapplinghook that's been spawned
  (`/Game/ExplosionsAndAction/Blueprints/Characters/BP_GrapplingHook.CloseGrapplingMovement` (`self.GrapplingHook`))
  (if (`/Game/ExplosionsAndAction/Blueprints/Characters/BP_GrapplingHook.HasNotHitAnything` (`self.GrapplingHook`))
    (`KismetSystemLibrary.Delay` (`self.GrapplingCooldown`)))
  (set `self.CanFireGrappling` true))

(event `self.EventWeaponFire`
  ;[1 1 1] Swing the weapon
  (if (`self.CanSwing`)
    (set `self.CanSwing` false)
    (bind _asweapon_base_class (cast `/Game/ExplosionsAndAction/Blueprints/Weapons/WeaponBaseClass` (`ChildActorComponent.ChildActor` (`self.PrimaryWeapon`))))
    (`/Game/ExplosionsAndAction/Blueprints/Weapons/WeaponBaseClass.Shoot` _asweapon_base_class false self)
    (`KismetSystemLibrary.Delay` (`self.SwingDelay`))
    (set `self.CanSwing` true)))

(event `self.LogDamage2`
  (params (Damage :type "Float (single-precision)"))
  (bind _asffaplayer_state (cast `/Game/ExplosionsAndAction/Blueprints/GameModes/FFAPlayerState` (`self.PlayerState`)))
  (`/Game/ExplosionsAndAction/Blueprints/GameModes/FFAPlayerState.UpdateClassStats` _asffaplayer_state 40 (`KismetMathLibrary.FFloor` Damage) 0))

(event `self.LogDeath2`
  (bind _asffaplayer_state (cast `/Game/ExplosionsAndAction/Blueprints/GameModes/FFAPlayerState` (`self.PlayerState`)))
  (`/Game/ExplosionsAndAction/Blueprints/GameModes/FFAPlayerState.UpdateClassStats` _asffaplayer_state 40 0 1))

(event `self.ReceiveTick`
  (params (DeltaSeconds :type "Float (single-precision)"))
  (bind _grapplinghook (`self.GrapplingHook`))
  (bind _grapplinghook_2 (`self.GrapplingHook`))
  (bind _hitcharacter (`/Game/ExplosionsAndAction/Blueprints/Characters/BP_GrapplingHook.HitCharacter` _grapplinghook))
  (bind _bhidden (`Actor.bHidden` (`ChildActorComponent.ChildActor` (`self.GrapplingRope`))))
  (`/Engine/EditorBlueprintResources/ActorMacros.Switch Has Authority`
    (:`Authority`
      (`/Engine/EditorBlueprintResources/StandardMacros.IsValid` _grapplinghook_2
        (:`Is Valid`
          (if (`/Game/ExplosionsAndAction/Blueprints/Characters/BP_GrapplingHook.ShouldRenderRope` _grapplinghook_2)
            (if _bhidden
              (`self.UpdateRopeHidden` false))
            (if (`/Game/ExplosionsAndAction/Blueprints/Characters/BP_GrapplingHook.HasNotHitAnything` _grapplinghook)
              (`self.UpdateRopeEndLocation` (`self.K2_GetActorLocation` _grapplinghook))
              (else
                (`/Engine/EditorBlueprintResources/StandardMacros.IsValid` _hitcharacter
                  (:`Is Valid`
                    (`self.UpdateRopeEndLocation` (`self.K2_GetActorLocation` _hitcharacter)))
                  (:`Is Not Valid`
                    (`self.UpdateRopeEndLocation` (`/Game/ExplosionsAndAction/Blueprints/Characters/BP_GrapplingHook.HitPosition` _grapplinghook))))))
            (elif (not _bhidden)
              (`self.UpdateRopeHidden` true))))))))

(event `UpdateRopeHidden`
  (params (Hidden :type Boolean :default false))
  (`self.SetActorHiddenInGame` (`ChildActorComponent.ChildActor` (`self.GrapplingRope`)) Hidden))

(event `UpdateRopeEndLocation`
  (params (EndLocation :type "Object.Vector Structure" :default (0.0 0.0 0.0)))
  (bind _returnvalue (`self.K2_GetActorLocation`))
  (bind _returnvalue_2 (`KismetMathLibrary.FindLookAtRotation` _returnvalue EndLocation))
  (`SceneComponent.K2_SetRelativeRotation` (select `bool` (> (.yaw (`self.GetControlRotation`)) 90.0) :`false` _returnvalue_2 :`true` (`KismetMathLibrary.ComposeRotators` (`KismetMathLibrary.MakeRot` 0.0 180.0) (* _returnvalue_2 -1.0))))
  (`SceneComponent.SetWorldScale3D` (`KismetMathLibrary.MakeVector` (/ (`KismetMathLibrary.VSize` (- EndLocation _returnvalue)) 100.0) 1.0 1.0)))

(fn `UserConstructionScript`
  (`parent.UserConstructionScript`)
  (`SceneComponent.SetVisibility` true)
  (`PrimitiveComponent.SetLockedAxis` (`self.CapsuleComponent`) "Y")
  (`PrimitiveComponent.SetLockedAxis` (`self.Sprite`) "Y")
  (`self.UpdateRopeHidden` true))