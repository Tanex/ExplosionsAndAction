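; Soldier character Blueprint that adds a fuel-limited jetpack and reports the class's deaths and damage taken.
; The fly event launches the character upward while fuel remains and upward speed is under a cap, draining fuel and playing a sustain sound.
; Tick refills fuel up to the maximum while the fly button is released, using tuning values set in the construction script.
; Logging events write class stats to the FFAPlayerState.
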(event `self.ReceiveBeginPlay`
  (`parent.ReceiveBeginPlay`))

(event `self.ReceiveActorBeginOverlap`
  (params (OtherActor :type "Actor Object Reference")))

(event `self.MovementFly`
  ;[1 1 1] Jetpack
  (if (> (`self.Jetpack Fuel`) (`self.Fuel Depletion`))
    (if (< (.z (`self.GetVelocity`)) 1000.0)
      (`self.LaunchCharacter` (0.0 0.0 400.0)))
    (set `self.Jetpack Fuel` (- (`self.Jetpack Fuel`) (`self.Fuel Depletion`)))
    (`self.PlaySound` "/Game/ExplosionsAndAction/Sounds/Soldier_JetPack_Sustain.Soldier_JetPack_Sustain")))

(event `self.ReceiveTick`
  (params (DeltaSeconds :type "Float (single-precision)"))
  ;[1 1 1] Jetpack Recharge
  (if (`self.FlyButtonPressed`)
    _
    (elif (< (`self.Jetpack Fuel`) (`self.Max Fuel`))
      (bind _output_get (set `self.Jetpack Fuel` (+ (* DeltaSeconds (`self.Fuel Recharge Rate`)) (`self.Jetpack Fuel`))))
      (if (> _output_get (`self.Max Fuel`))
        (set `self.Jetpack Fuel` (`self.Max Fuel`))))))

(event `self.LogDeath2`
  ;[1 1 1] Handles logging
  (bind _asffaplayer_state (cast `/Game/ExplosionsAndAction/Blueprints/GameModes/FFAPlayerState` (`self.PlayerState`)))
  (`/Game/ExplosionsAndAction/Blueprints/GameModes/FFAPlayerState.UpdateClassStats` _asffaplayer_state 10 0 1))

(event `self.LogDamage2`
  (params (Damage :type "Float (single-precision)"))
  ;[1 1 1] Handles logging
  (bind _asffaplayer_state (cast `/Game/ExplosionsAndAction/Blueprints/GameModes/FFAPlayerState` (`self.PlayerState`)))
  (`/Game/ExplosionsAndAction/Blueprints/GameModes/FFAPlayerState.UpdateClassStats` _asffaplayer_state 10 (`KismetMathLibrary.FFloor` Damage) 0))

(fn `UserConstructionScript`
  (`parent.UserConstructionScript`)
  (bind _output_get (set `self.Max Fuel` 80.0))
  (set `self.Jetpack Fuel` _output_get)
  (set `self.Fuel Depletion` 4.5)
  (set `self.Fuel Recharge Rate` 10.0))