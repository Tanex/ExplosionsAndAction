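; Grappling hook actor that pulls its instigator toward what it hits, constrained to the X-Z plane.
; On the server, the first valid overlap hides the hook and opens movement gates; hit characters or pickups take damage and are also pulled toward the instigator.
; Self-repeating timers reapply launches or impulses through the gates until the dead zone is reached.
; Closing, also triggered by a miss timeout, shuts the gates and expires the actor.
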(event `MaxRangeReached`
  (if (`self.HasNotHitAnything`)
    (`self.CloseGrapplingMovement`)))

(event `self.RenderComponent.OnComponentBeginOverlap`
  (params (OtherActor :type "Actor Object Reference") (OtherComp :type "PrimitiveComponent Object Reference") (OtherBodyIndex :type Integer) (bFromSweep :type Boolean) (SweepResult :type "EngineTypes.HitResult Structure (by ref)"))
  (bind _returnvalue (`self.GetInstigator`))
  (bind _returnvalue_2 (`GameplayStatics.GetObjectClass` OtherActor))
  (`/Engine/EditorBlueprintResources/ActorMacros.Switch Has Authority`
    (:`Authority`
      (if (and (not (`self.ActorHasTag` OtherActor "NoBulletCollide")) (`self.HasNotHitAnything`) (!= OtherActor _returnvalue) (select `bool` (`KismetMathLibrary.ClassIsChildOf` (`GameplayStatics.GetObjectClass` OtherActor) "/Game/ExplosionsAndAction/Blueprints/Blocks/BP_BaseBlock.BP_BaseBlock_C") :`false` true :`true` (!= _returnvalue (`ActorComponent.GetOwner` (`SceneComponent.GetAttachParent` (`self.K2_GetRootComponent` OtherActor))))))
        (set `self.HasNotHitAnything` false)
        (`self.SetActorHiddenInGame` true)
        (`self.OpenGrapplingMovement`)
        (if (or (`KismetMathLibrary.ClassIsChildOf` _returnvalue_2 "/Game/ExplosionsAndAction/Blueprints/Characters/BP_BaseCharacter.BP_BaseCharacter_C") (== _returnvalue_2 "/Game/ExplosionsAndAction/Blueprints/PickupBlueprint.PickupBlueprint_C"))
          (bind _output_get (set `self.HitCharacter` OtherActor))
          (`GameplayStatics.ApplyDamage` _output_get 5.0 (`self.GetInstigatorController`) self "/Script/Engine.DamageType")
          (`self.CharacterWasHit`)
          (else
            (set `self.HitPosition` (`self.K2_GetActorLocation`))
            (`self.WorldWasHit`)))))))

(event `WorldWasHit`
  (bind _hitposition (`self.HitPosition`))
  ;[1 1 1] The world was hit, pull the instigator towards the hit position
  (`/Engine/EditorBlueprintResources/StandardMacros.Gate` true :!label _label
    (:`Exit`
      (`/Engine/EditorBlueprintResources/ActorMacros.Switch Has Authority`
        (:`Authority`
          (bind _asbp_base_character (cast `/Game/ExplosionsAndAction/Blueprints/Characters/BP_BaseCharacter` (`self.GetInstigator`)))
          (bind _returnvalue (`self.K2_GetActorLocation` _asbp_base_character))
          (if (> (`KismetMathLibrary.VSize` (- _hitposition _returnvalue)) (`self.GrapplingDeadZone`))
            (`Character.LaunchCharacter` _asbp_base_character (* (`KismetMathLibrary.GreaterGreater_VectorRotator` (`KismetMathLibrary.MakeVector` (`self.GrapplingSpeed`)) (`KismetMathLibrary.FindLookAtRotation` _returnvalue _hitposition)) (1.0 0.0 1.0)) false false)
            (`KismetSystemLibrary.K2_SetTimer` null "WorldWasHit" 0.1)
            (else
              (`self.CloseGrapplingMovement`))))))))

(event `OpenGrapplingMovement`
  (bind _hitcharacter (`self.HitCharacter`))
  (bind _returnvalue (`self.K2_GetActorLocation` (`self.HitCharacter`)))
  ;[1 1 1] Enable pulling with the grappling hook
  (`|ExecutionSequence`
    (:`then_0`
      (goto _label :!via `Open`))
    (:`then_1`
      (goto _label_2 :!via `Open`))))

(event `CloseGrapplingMovement`
  (bind _hitcharacter (`self.HitCharacter`))
  (bind _returnvalue (`self.K2_GetActorLocation` (`self.HitCharacter`)))
  ;[1 1 1] Disable and remove the grappling hook
  (`|ExecutionSequence`
    (:`then_0`
      (goto _label :!via `Close`))
    (:`then_1`
      (goto _label_2 :!via `Close`))
    (:`then_2`
      (set `self.ShouldRenderRope` false)
      (set `PrimitiveComponent.bGenerateOverlapEvents` false (`self.RenderComponent`))
      (`self.SetActorHiddenInGame` true)
      (`self.SetLifeSpan` 2.0))))

(event `CharacterWasHit`
  (bind _hitcharacter (`self.HitCharacter`))
  (bind _returnvalue (`self.K2_GetActorLocation` (`self.HitCharacter`)))
  ;[1 1 1] Another character was hit, pull both characters towards each other
  (`/Engine/EditorBlueprintResources/StandardMacros.Gate` true :!label _label_2
    (:`Exit`
      (`/Engine/EditorBlueprintResources/ActorMacros.Switch Has Authority`
        (:`Authority`
          (bind _asbp_base_character (cast `/Game/ExplosionsAndAction/Blueprints/Characters/BP_BaseCharacter` (`self.GetInstigator`)))
          (bind _returnvalue_2 (`self.K2_GetActorLocation` _asbp_base_character))
          (if (> (`KismetMathLibrary.VSize` (- _returnvalue _returnvalue_2)) (`self.GrapplingDeadZone`))
            (`Character.LaunchCharacter` _asbp_base_character (* (`KismetMathLibrary.GreaterGreater_VectorRotator` (`KismetMathLibrary.MakeVector` (`self.GrapplingSpeed`)) (`KismetMathLibrary.FindLookAtRotation` _returnvalue_2 _returnvalue)) (1.0 0.0 1.0)) false false)
            (bind _asbp_base_character_2 (cast `/Game/ExplosionsAndAction/Blueprints/Characters/BP_BaseCharacter` _hitcharacter)
              (:`then`
                (bind _returnvalue_3 (* (`KismetMathLibrary.GreaterGreater_VectorRotator` (2000.0 0.0 0.0) (`KismetMathLibrary.FindLookAtRotation` _returnvalue _returnvalue_2)) (1.0 0.0 1.0)))
                (`Character.LaunchCharacter` _asbp_base_character_2 _returnvalue_3 false false))
              (:`CastFailed`
                (bind _aspickup_blueprint (cast `/Game/ExplosionsAndAction/Blueprints/PickupBlueprint` _hitcharacter))
                (`PrimitiveComponent.AddImpulse` _aspickup_blueprint _returnvalue_3 "None" true)))
            (`KismetSystemLibrary.K2_SetTimer` null "CharacterWasHit" 0.1)
            (else
              (`self.CloseGrapplingMovement`))))))))

(fn `UserConstructionScript`
  (`/Engine/EditorBlueprintResources/ActorMacros.Switch Has Authority`
    (:`Authority`
      (`KismetSystemLibrary.K2_SetTimer` null "MaxRangeReached" (`self.GrapplingLifeTime`)))))