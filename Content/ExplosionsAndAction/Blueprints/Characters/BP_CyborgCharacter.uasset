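; Playable 2D Cyborg character class with a fuel-limited jetpack that launches it toward the mouse location.
; The fly event spends fuel, launches the character in the XZ plane and pauses recharging.
; Tick refills fuel on the authority only, resuming once the character can jump.
; It also picks idle, move or jump flipbooks and reports damage and deaths to the FFA player state's class stats.
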(event `self.ReceiveBeginPlay`
  (`parent.ReceiveBeginPlay`))

(event `self.ReceiveActorBeginOverlap`
  (params (OtherActor :type "Actor Object Reference")))

(event `self.ReceiveTick`
  (params (DeltaSeconds :type "Float (single-precision)"))
  (bind _max_fuel (`self.Max Fuel`))
  (`parent.ReceiveTick` DeltaSeconds)
  (`/Engine/EditorBlueprintResources/ActorMacros.Switch Has Authority`
    (:`Authority`
      (if (< (`self.Jetpack Fuel`) (`self.Max Fuel`))
        (if (`self.DoFuelRecharge`)
          (bind _output_get (set `self.Jetpack Fuel` (+ (`self.Jetpack Fuel`) (* (`self.Fuel Recharge Rate`) DeltaSeconds))))
          (if (> _output_get _max_fuel)
            (set `self.Jetpack Fuel` _max_fuel))
          (elif (`self.CanJump`)
            (set `self.DoFuelRecharge` true)))))))

(event `self.EventStartFly`
  (params (MouseLocation :type "Object.Vector Structure"))
  (if (>= (`self.Jetpack Fuel`) (`self.Fuel Depletion`))
    (set `self.Jetpack Fuel` (- (`self.Jetpack Fuel`) (`self.Fuel Depletion`)))
    (set `self.DoFuelRecharge` false)
    (`self.LaunchCharacter` (* (`KismetMathLibrary.GreaterGreater_VectorRotator` (2000.0 0.0 0.0) (`KismetMathLibrary.FindLookAtRotation` (`self.K2_GetActorLocation`) MouseLocation)) (1.0 0.0 1.0)) true true)
    (`self.PlaySound` "/Game/ExplosionsAndAction/Sounds/Soldier_JetPack_Off.Soldier_JetPack_Off")))

(event `self.AnimationUpdate`
  (`PaperFlipbookComponent.SetFlipbook` (`self.Sprite`) (select `bool` (`NavMovementComponent.IsMovingOnGround` (`self.CharacterMovement`)) :`false` "/Game/ExplosionsAndAction/Textures/CyborgJump.CyborgJump" :`true` (select `bool` (> (`KismetMathLibrary.VSize` (`self.GetVelocity`)) 0.0) :`false` "/Game/ExplosionsAndAction/Textures/CyborgIdle.CyborgIdle" :`true` "/Game/ExplosionsAndAction/Textures/CyborgMove.CyborgMove" :!type "PaperFlipbook Object Reference"))))

(event `self.LogDamage2`
  (params (Damage :type "Float (single-precision)"))
  (bind _asffaplayer_state (cast `/Game/ExplosionsAndAction/Blueprints/GameModes/FFAPlayerState` (`self.PlayerState`)))
  (`/Game/ExplosionsAndAction/Blueprints/GameModes/FFAPlayerState.UpdateClassStats` _asffaplayer_state 20 (`KismetMathLibrary.FFloor` Damage) 0))

(event `self.LogDeath2`
  (bind _asffaplayer_state (cast `/Game/ExplosionsAndAction/Blueprints/GameModes/FFAPlayerState` (`self.PlayerState`)))
  (`/Game/ExplosionsAndAction/Blueprints/GameModes/FFAPlayerState.UpdateClassStats` _asffaplayer_state 20 0 1))

(fn `UserConstructionScript`
  (`parent.UserConstructionScript`)
  (bind _output_get (set `self.Max Fuel` 90.0))
  (set `self.Jetpack Fuel` _output_get)
  (set `self.Fuel Depletion` 45.0)
  (set `self.Fuel Recharge Rate` 150.0)
  (`SceneComponent.SetRelativeScale3D` (3.5 3.5 4.0))
  (`SceneComponent.SetRelativeScale3D` (1.0 1.0 1.0)))