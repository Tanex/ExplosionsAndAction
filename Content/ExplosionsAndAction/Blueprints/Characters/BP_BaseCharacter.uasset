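; Base 2D flipbook character for a free-for-all shooter, handling movement, animation, blocking, health, weapons and death.
; Input events forward to primary and secondary child-actor weapons through GetActiveWeapon, mirroring ammo and reload progress into UI variables.
; Damage spawns floating text via the attacker's character, while death hides the character and adjusts player-state scores, penalizing self-kills.
; A gated DelayedTrigger macro repeats flying while held, though MovementFly is empty.
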(event Custom|EventWeaponFire
  ;[1 1 1] Event that handles firing the weapon
  (Variables|InputStates|SetFireButtonPressed true)
  (bind _weapon (CallFunction|GetActiveWeapon))
  (Default|Shoot _weapon (Variables|InputStates|GetFireButtonPressed) self))

(event Custom|UpdateAmmoInMag
  ;[1 1 1] Updating variables for UI
  (bind _weapon (CallFunction|GetActiveWeapon))
  (Variables|Weapon|SetAmmoInMag (Variables|/Game/ExplosionsAndAction/Blueprints/Weapons/WeaponBaseClass.WeaponBaseClass_C|GetAmmoInMagazine _weapon))
  (Variables|Weapon|SetAmmo (Variables|/Game/ExplosionsAndAction/Blueprints/Weapons/WeaponBaseClass.WeaponBaseClass_C|GetAvailableAmmo _weapon)))

(event Custom|EventStopWeaponFire
  ;[1 1 1] Event that handles firing the weapon
  (Variables|InputStates|SetFireButtonPressed false)
  (bind _weapon (CallFunction|GetActiveWeapon))
  (Default|Shoot _weapon (Variables|InputStates|GetFireButtonPressed) self))

(event Custom|KillCharacter
  (params (Instigator :type Controller%20Object%20Reference))
  (Rendering|SetActorHiddenInGame true)
  (bind (_primaryweapon _secondaryweapon) (Utilities|GetWeapons self)
    (:Out
      (Rendering|SetActorHiddenInGame _primaryweapon true)
      (Rendering|SetActorHiddenInGame _secondaryweapon true)
      (CallFunction|PlaySound "/Game/ExplosionsAndAction/Sounds/Soldier_Death_var3.Soldier_Death_var3")
      (CallFunction|RemoveAllAmmo)
      (Collision|SetActorEnableCollision false)
      (Actor|SetLifeSpan 1.0)
      (Variables|/Script/Engine.MovementComponent|SetVelocity (Variables|Character|GetCharacterMovement) "0, 0, 0")
      (if (== Instigator (Pawn|GetController))
        (bind _asffaplayer_state (Utilities|Casting|CastToFFAPlayerState (Variables|GetPlayerState) :!label _label))
        (Variables|/Game/ExplosionsAndAction/Blueprints/GameModes/FFAPlayerState.FFAPlayerState_C|SetPlayerScore _asffaplayer_state (- (Variables|/Game/ExplosionsAndAction/Blueprints/GameModes/FFAPlayerState.FFAPlayerState_C|GetPlayerScore _asffaplayer_state) 1))
        (else
          (bind _asffaplayer_state_2 (Utilities|Casting|CastToFFAPlayerState (Variables|/Script/Engine.Controller|GetPlayerState Instigator))
            (:then
              (Variables|/Game/ExplosionsAndAction/Blueprints/GameModes/FFAPlayerState.FFAPlayerState_C|SetPlayerScore _asffaplayer_state_2 (+ (Variables|/Game/ExplosionsAndAction/Blueprints/GameModes/FFAPlayerState.FFAPlayerState_C|GetPlayerScore _asffaplayer_state_2) 1)))
            (:CastFailed
              (goto _label))))))))

(event Custom|EventStartFly
  (Variables|InputStates|SetFlyButtonPressed true)
  (Utilities|DelayedTrigger (stale Custom|EventStopFly _output_get) (Variables|Movement|GetFlyingDelay)
    (:TriggeredFunction
      (Movement|MovementFly))))

(event Custom|ChangeWeaponOffsetLeft
  ;[1 1 1] Handles Weapon Rotation and Offset
  (Transformation|SetRelativeLocation "0,-0.100000, 0" false)
  (Transformation|SetRelativeLocation "0,-0.100000, 0" false))

(event Custom|EventStopFly
  (bind _output_get (Variables|InputStates|SetFlyButtonPressed false))
  (Utilities|DelayedTrigger _output_get (Variables|Movement|GetFlyingDelay)
    (:TriggeredFunction
      (Movement|MovementFly))))

(event Custom|UpdateReloadProg
  ;[1 1 1] Updating variables for UI
  (bind _weapon (CallFunction|GetActiveWeapon))
  (Variables|Default|SetReloadProg (Variables|/Game/ExplosionsAndAction/Blueprints/Weapons/WeaponBaseClass.WeaponBaseClass_C|GetReloadProgress _weapon)))

(event Custom|RotateWeapon
  (params (WeaponRotation :type Rotator :default "0, 0, 0"))
  ;[1 1 1] Handles Weapon Rotation and Offset
  (Transformation|SetRelativeRotation WeaponRotation false)
  (Transformation|SetRelativeRotation WeaponRotation false))

(event Custom|PlaySound
  (params (Sound :type Sound%20Wave%20Object%20Reference))
  ;[1 1 1] Event that handles playing sounds
  (Audio|PlaySoundatLocation Sound (Transformation|GetActorLocation) 1.0 1.0 0.0 "/Game/ExplosionsAndAction/Sounds/Settings.Settings"))

(event Custom|EventSpawnDamageText
  (params (Location :type Transform) (Damage :type Float%20%28single-precision%29 :default 0.0))
  (bind _returnvalue (Game|SpawnActorfromClass "/Game/ExplosionsAndAction/Blueprints/BP_FloatingDamageText.BP_FloatingDamageText_C" Location false 0))
  (Development|PrintText "Hello")
  (Default|Initializer _returnvalue Damage)
  (bind _asbase_player_controller (Utilities|Casting|CastToBasePlayerController (Pawn|GetController)))
  (Variables|/Game/ExplosionsAndAction/Blueprints/Controllers/BasePlayerController.BasePlayerController_C|SetHasHitSomething _asbase_player_controller true)
  (Utilities|FlowControl|RetriggerableDelay 0.3)
  (Variables|/Game/ExplosionsAndAction/Blueprints/Controllers/BasePlayerController.BasePlayerController_C|SetHasHitSomething _asbase_player_controller false))

(event Custom|UpdateAnimation
  ;[1 1 1] Handle animation updates
  (CallFunction|AnimationUpdate))

(event Custom|ReloadWeapon
  (bind _weapon (CallFunction|GetActiveWeapon))
  (Default|ReloadWeapon _weapon self))

(event Custom|ChangeWeaponOffsetRight
  ;[1 1 1] Handles Weapon Rotation and Offset
  (Transformation|SetRelativeLocation "0,0.100000, 0" false)
  (Transformation|SetRelativeLocation "0,0.100000, 0" false))

(event Custom|SwapWeapon
  ;[1 1 1] Changes Active Weapon on a Player
  (CallFunction|EventStopWeaponFire)
  (switch int (Variables|Weapon|GetActiveWeapon)
    (:1
      (Variables|Weapon|SetActiveWeapon 2))
    (:2
      (Variables|Weapon|SetActiveWeapon 1)))
  (CallFunction|UpdateAmmoinMag))

(event EventAnyDamage
  (params (Damage :type Float%20%28single-precision%29) (DamageType :type Damage%20Type%20Object%20Reference) (InstigatedBy :type Controller%20Object%20Reference) (DamageCauser :type Actor%20Object%20Reference))
  (bind _output_get (Variables|StateVariables|SetHealth (- (Variables|StateVariables|GetHealth) Damage)))
  (Utilities|SpawnDamageText Damage InstigatedBy
    (:Out
      (CallFunction|PlaySound "/Game/ExplosionsAndAction/Sounds/Soldier_Take_Damage_var1.Soldier_Take_Damage_var1")
      (if (<= _output_get 0.0)
        (CallFunction|KillCharacter InstigatedBy)))))

(event EventTick
  (params (DeltaSeconds :type Float%20%28single-precision%29))
  (CallFunction|UpdateReloadProg))

(event EventBeginPlay
  ;[1 1 1] Comment
  (CallFunction|UpdateAmmoinMag))

(fn ConstructionScript
  (bind _maxhealth (Variables|Attributes|GetMaxHealth))
  (Variables|StateVariables|SetHealth _maxhealth)
  (Variables|StateVariables|SetHealthPercent _maxhealth)
  (Transformation|SetWorldScale3D "3.450000,3.450000,3.450000")
  ;[1 1 1] Set Components to Replicate
  (Class|ActorComponent|SetIsReplicated true)
  (Class|ActorComponent|SetIsReplicated true)
  (Class|ActorComponent|SetIsReplicated true)
  (Rendering|SetVisibility false true))

(fn MovementHorizontal
  (params (Direction :type Float%20%28single-precision%29 :default 0.0))
  (Pawn|Input|AddMovementInput "1.000000,0.000000, 0" Direction false)
  (CallFunction|UpdateAnimation))

(fn MovementJump
  (if (Variables|InputStates|GetJumpButtonPressed)
    (Character|Jump)
    (if (Character|CanJump)
      (CallFunction|PlaySound "/Game/ExplosionsAndAction/Sounds/Soldier_Jump_var1.Soldier_Jump_var1"))
    (else
      (Character|StopJumping))))

(fn MovementBlock
  (bind _asbp_base_block (Utilities|Casting|CastToBP_BaseBlock (Variables|/Script/Engine.ChildActorComponent|GetChildActor (Variables|Default|GetBlock))))
  (if (Variables|InputStates|GetBlockButtonPressed)
    (Default|BlockPressed _asbp_base_block)
    (else
      (Default|BlockReleased _asbp_base_block))))

(fn WeaponSwap
  (Rendering|ToggleVisibility true)
  (Rendering|ToggleVisibility true)
  (CallFunction|SwapWeapon))

(fn AnimationUpdate
  (Sprite|SetFlipbook (Variables|Default|GetSprite) (select (AI|Components|NavMovement|IsMovingonGround) (select (> (Math|Vector|VectorLength (Transformation|GetVelocity)) 0.0) "/Game/ExplosionsAndAction/Sprites/SoldierClass/SoldierRun.SoldierRun" "/Game/ExplosionsAndAction/Sprites/SoldierClass/SoldierIdle.SoldierIdle") "/Game/ExplosionsAndAction/Sprites/SoldierClass/SoldierJump.SoldierJump")))

(fn ServerFireBullet)

(fn InitAttributes
  (Variables|StateVariables|SetHealth (Variables|Attributes|GetMaxHealth)))

(fn MovementFly)

(fn GetActiveWeapon
  (Math|Integer|CompareInt (Variables|Weapon|GetActiveWeapon) 1
    (:>
      (bind _asweapon_base_class (Utilities|Casting|CastToWeaponBaseClass (Variables|/Script/Engine.ChildActorComponent|GetChildActor (Variables|Default|GetSecondaryWeapon)))
        (:then
          (LocalVariables|SetCurrentWeapon _asweapon_base_class))
        (:CastFailed
          (LocalVariables|SetCurrentWeapon 0 :!label _label))))
    (:==
      (bind _asweapon_base_class_2 (Utilities|Casting|CastToWeaponBaseClass (Variables|/Script/Engine.ChildActorComponent|GetChildActor (Variables|Default|GetPrimaryWeapon)))
        (:then
          (LocalVariables|SetCurrentWeapon _asweapon_base_class_2))
        (:CastFailed
          (goto _label)))))
  (return (LocalVariables|GetCurrentWeapon)))

(fn RemoveAllAmmo
  (bind (_primaryweapon _secondaryweapon) (Utilities|GetWeapons self)
    (:Out
      (Variables|/Game/ExplosionsAndAction/Blueprints/Weapons/WeaponBaseClass.WeaponBaseClass_C|SetAmmoInMagazine _primaryweapon 0)
      (Variables|/Game/ExplosionsAndAction/Blueprints/Weapons/WeaponBaseClass.WeaponBaseClass_C|SetAvailableAmmo _primaryweapon 0)
      (Variables|/Game/ExplosionsAndAction/Blueprints/Weapons/WeaponBaseClass.WeaponBaseClass_C|SetAmmoInMagazine _secondaryweapon 0)
      (Variables|/Game/ExplosionsAndAction/Blueprints/Weapons/WeaponBaseClass.WeaponBaseClass_C|SetAvailableAmmo _secondaryweapon 0))))