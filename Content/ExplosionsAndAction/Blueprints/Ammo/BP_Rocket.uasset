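; BP_Rocket is a rocket ammo Blueprint that deals explosive area damage.
; Its DoDamage event applies radial damage with falloff at the actor's location, with inner and outer radii, the instigator's controller and WorldStatic as the blocking channel.
; It then calls SpawnExplosion, which spawns the explosion particle emitter at that point with a fixed rotation.
; Nothing in this graph calls DoDamage, and the construction script only runs the parent's.
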(event `self.DoDamage`
  (params (`Other Actor` :type "Actor Object Reference"))
  (bind _returnvalue (`self.K2_GetActorLocation`))
  (`GameplayStatics.ApplyRadialDamageWithFalloff` :`BaseDamage` (`self.Damage`) :`Origin` _returnvalue :`DamageInnerRadius` (`self.InnerRadius`) :`DamageOuterRadius` (`self.OuterRadius`) :`DamageFalloff` (`self.Falloff`) :`DamageTypeClass` "/Script/Engine.DamageType" :`DamageCauser` self :`InstigatedByController` (`self.GetInstigatorController`) :`DamagePreventionChannel` "ECC_WorldStatic")
  (`self.SpawnExplosion` _returnvalue))

(event `SpawnExplosion`
  (params (Location :type "Object.Vector Structure" :default (0.0 0.0 0.0)))
  (`GameplayStatics.SpawnEmitterAtLocation` "/Game/ExplosionsAndAction/Particles/Explosion/Explosion.Explosion" Location (struct :`Yaw` 270.0)))

(fn `UserConstructionScript`
  (`parent.UserConstructionScript`))