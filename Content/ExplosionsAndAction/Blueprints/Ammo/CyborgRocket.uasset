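; CyborgRocket is a rocket projectile ammo Blueprint that inherits damage and hit logic from a parent class.
; Its construction script sets the weapon ID, runs the parent construction script, then tunes damage radius, falloff and launch speed.
; Three seconds after BeginPlay, an unhit rocket calls DoDamage, disables overlaps and collision, hides itself and sets a short lifespan for cleanup.
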(event `self.ReceiveBeginPlay`
  (`KismetSystemLibrary.Delay` 3.0)
  (if (`self.HasNotHitAnything`)
    (set `self.HasNotHitAnything` false)
    (`self.DoDamage` null)
    (set `PrimitiveComponent.bGenerateOverlapEvents` false (`self.RenderComponent`))
    (`self.SetActorEnableCollision` false)
    (`self.SetActorHiddenInGame` true)
    (`self.SetLifeSpan` 2.0)))

(event `self.ReceiveActorBeginOverlap`
  (params (OtherActor :type "Actor Object Reference")))

(event `self.ReceiveTick`
  (params (DeltaSeconds :type "Float (single-precision)")))

(fn `UserConstructionScript`
  (set `self.WeaponId` 21)
  (`parent.UserConstructionScript`)
  (set `self.InnerRadius` 80.0)
  (set `self.Falloff` 2.0)
  (set `ProjectileMovementComponent.InitialSpeed` 1400.0 (`self.ProjectileMovement`)))