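; Base ammo Blueprint for projectiles that deal damage to the first valid actor they overlap.
; Construction sets a lifespan to clear stray bullets and doubles damage if the instigating character's PickupHandler has double damage.
; On server-side overlap it ignores tagged actors, the instigator and the instigator's own blocks.
; A valid hit applies damage with slight random variance, then disables collision, hides the bullet and shortens its lifespan.
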(event `self.RenderComponent.OnComponentBeginOverlap`
  (params (OtherActor :type "Actor Object Reference") (OtherComp :type "PrimitiveComponent Object Reference") (OtherBodyIndex :type Integer) (bFromSweep :type Boolean) (SweepResult :type "EngineTypes.HitResult Structure (by ref)"))
  (bind _returnvalue (`self.GetInstigator`))
  ;[1 1 1] Do damage on hit
  (`/Engine/EditorBlueprintResources/ActorMacros.Switch Has Authority`
    (:`Authority`
      (if (and (not (`self.ActorHasTag` OtherActor "NoBulletCollide")) (`self.HasNotHitAnything`) (!= OtherActor _returnvalue) (select `bool` (`KismetMathLibrary.ClassIsChildOf` (`GameplayStatics.GetObjectClass` OtherActor) "/Game/ExplosionsAndAction/Blueprints/Blocks/BP_BaseBlock.BP_BaseBlock_C") :`false` true :`true` (!= _returnvalue (`ActorComponent.GetOwner` (`SceneComponent.GetAttachParent` (`self.K2_GetRootComponent` OtherActor))))))
        (set `self.HasNotHitAnything` false)
        (`self.DoDamage` OtherActor)
        (set `PrimitiveComponent.bGenerateOverlapEvents` false (`self.RenderComponent`))
        (`self.SetActorEnableCollision` false)
        (`self.SetActorHiddenInGame` true)
        (`self.SetLifeSpan` 2.0)))))

(fn `DoDamage`
  (params (`Other Actor` :type "Actor Object Reference"))
  (`GameplayStatics.ApplyDamage` `Other Actor` (* (`KismetMathLibrary.RandomFloatInRange` 0.9 1.1) (`self.Damage`)) (`self.GetInstigatorController`) self (`self.DamageType`)))

(fn `UserConstructionScript`
  ;[1 1 1] Make sure stray bullets are destroyed
  (`self.SetLifeSpan` 10.0)
  (`SceneComponent.SetWorldScale3D` (1.0 1.0 1.0))
  ;[1 1 1] Check double damage
  (bind _asbp_base_character (cast `/Game/ExplosionsAndAction/Blueprints/Characters/BP_BaseCharacter` (`self.GetInstigator`)))
  (if (`/Game/ExplosionsAndAction/Blueprints/Characters/PickupHandler.HasDoubleDamage` (`/Game/ExplosionsAndAction/Blueprints/Characters/BP_BaseCharacter.PickupHandler` _asbp_base_character))
    (set `self.Damage` (* (`self.Damage`) 2.0))))