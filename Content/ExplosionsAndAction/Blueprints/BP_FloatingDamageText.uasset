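; Floating damage number actor that shows a damage value as text drifting upward in the world.
; Initializer sets the DamageText component to the damage rounded down to a whole number.
; The construction script applies a fixed rotation and sets the lifespan from VisibleTime, so the actor removes itself.
; Tick moves it along world Z at FloatSpeed, scaled by delta time and without sweeping.
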(event `self.ReceiveTick`
  (params (DeltaSeconds :type "Float (single-precision)"))
  (`self.K2_SetActorLocation` (+ (`KismetMathLibrary.MakeVector` 0.0 0.0 (* DeltaSeconds (`self.FloatSpeed`))) (`self.K2_GetActorLocation`))))

(fn `Initializer`
  (params (Damage :type "Float (double-precision)"))
  (`TextRenderComponent.SetText` (`self.DamageText`) (`KismetStringLibrary.Conv_IntToString` (`KismetMathLibrary.FFloor` Damage))))

(fn `UserConstructionScript`
  (`self.SetActorRotation` (struct :`Yaw` 90.0))
  (`self.SetLifeSpan` (`self.VisibleTime`)))