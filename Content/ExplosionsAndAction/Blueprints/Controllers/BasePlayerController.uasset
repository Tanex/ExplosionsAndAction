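; Player controller for a side-view multiplayer shooter, linking input to the controlled BP_BaseCharacter and game UI.
; Tick flips facing and rotates the weapon toward the deprojected mouse cursor on the XZ plane.
; Input handlers forward movement, jump/block, flight and weapon actions through macros that lazily cache the character.
; Menus and log messages route through BaseGameInstance, respawns through BaseGameMode on authority, and suicide applies lethal damage.
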(event `Request Player Name`
  ;[1 1 1] Set Name
  (bind _asbase_game_instance (cast `/Game/ExplosionsAndAction/Blueprints/BaseGameInstance` (`GameplayStatics.GetGameInstance`)))
  (`self.SetPlayerName` (`/Game/ExplosionsAndAction/Blueprints/BaseGameInstance.PlayerName` _asbase_game_instance)))

(event `InputAction|Menu`
  ;[1 1 1] Pause Menu
  (:`Pressed`
    (bind _asbase_game_instance (cast `/Game/ExplosionsAndAction/Blueprints/BaseGameInstance` (`GameplayStatics.GetGameInstance`)))
    (`/Game/ExplosionsAndAction/Blueprints/BaseGameInstance.ShowPauseMenu` _asbase_game_instance)))

(event `SetPlayerName`
  (params (PlayerName :type Text))
  ;[1 1 1] Set Name
  (bind _asffaplayer_state (cast `/Game/ExplosionsAndAction/Blueprints/GameModes/FFAPlayerState` (`self.PlayerState`)))
  (set `/Game/ExplosionsAndAction/Blueprints/GameModes/FFAPlayerState.Name` PlayerName _asffaplayer_state))

(event `self.ReceiveBeginPlay`
  ;[1 1 1] Begin Play
  (set `self.HasHitSomething` false)
  (`self.Request Player Name`)
  (`self.BindOnDestroyed`)
  (`self.ShowSpawnMenu`))

(event `BindOnDestroyed`
  (bind _returnvalue (`self.K2_GetPawn`))
  ;[1 1 1] Bind SpawnMenu to OnDestroyed
  (`/Engine/EditorBlueprintResources/StandardMacros.IsValid` _returnvalue
    (:`Is Valid`
      (add `self.OnDestroyed` _returnvalue (delegate `OnDestroyedEvent`)))))

(event `OnDestroyedEvent`
  ;[1 1 1] Show SpawnMenu when destroyed
  (`/Engine/EditorBlueprintResources/ActorMacros.Switch Has Authority`
    (:`Authority`
      (`self.ShowSpawnMenu`))))

(event `self.ReceiveTick`
  (params (DeltaSeconds :type "Float (single-precision)"))
  (bind _controlledcharacter (`self.ControlledCharacter`))
  ;[1 1 1] Handle Everything affected by cursor position
  (if (`self.IsLocalPlayerController`)
    (`self.GetControlledCharIfInvalid`
      (:`Out`
        (`self.GetMouseFlip`
          (:`FaceRight`
            (`self.SetControlRotation` (`KismetMathLibrary.MakeRot` 0.0 0.0))
            (`/Game/ExplosionsAndAction/Blueprints/Characters/BP_BaseCharacter.ChangeWeaponOffsetRight` _controlledcharacter))
          (:`FaceLeft`
            (`self.SetControlRotation` (`KismetMathLibrary.MakeRot` 0.0 180.0))
            (`/Game/ExplosionsAndAction/Blueprints/Characters/BP_BaseCharacter.ChangeWeaponOffsetLeft` _controlledcharacter))
          (:`Out`
            (bind _weaponrotation (`self.WeaponRotation`)
              (:`Out`
                (`/Game/ExplosionsAndAction/Blueprints/Characters/BP_BaseCharacter.RotateWeapon` (`self.ControlledCharacter`) _weaponrotation)))))))))

(event `InitSpawnMenu`
  ;[1 1 1] Show Spawn Menu
)

(event `ShowSpawnMenu`
  ;[1 1 1] Show Spawn Menu
  (bind _asbase_game_instance (cast `/Game/ExplosionsAndAction/Blueprints/BaseGameInstance` (`GameplayStatics.GetGameInstance`)))
  (`/Game/ExplosionsAndAction/Blueprints/BaseGameInstance.ShowSpawnMenu` _asbase_game_instance)
  (set `self.CurrentPlayingState` "NewEnumerator1"))

(event `InputAxis|MoveRight`
  (params (AxisValue :type "Float (single-precision)"))
  (bind _controlledcharacter (`self.ControlledCharacter`))
  ;[1 1 1] Handles Horizontal Movement Input
  (`self.GetControlledCharIfInvalid`
    (:`Out`
      (if (`/Game/ExplosionsAndAction/Blueprints/Characters/BP_BaseCharacter.InputEnabled` _controlledcharacter)
        (`/Game/ExplosionsAndAction/Blueprints/Characters/BP_BaseCharacter.MovementHorizontal` _controlledcharacter AxisValue)))))

(event `EventRequestRespawn`
  (params (ClassType :type "/Game/ExplosionsAndAction/Blueprints/Characters/CharacterTypes Enum" :default "NewEnumerator0"))
  ;[1 1 1] Request Respawn
  (if (`self.IsLocalPlayerController`)
    (`/Engine/EditorBlueprintResources/StandardMacros.IsValid` (`self.K2_GetPawn`)
      (:`Is Not Valid`
        (`self.requestServerRespawn` ClassType)
        (set `self.CurrentPlayingState` "NewEnumerator0")))))

(event `InputAxis|JumpBlock`
  (params (AxisValue :type "Float (single-precision)"))
  ;[1 1 1] Comment
  (if (!= AxisValue 0.0)
    (if (> AxisValue 0.0)
      ;[1 1 1] Handles Jump Input
      (set `self.JumpLast` true)
      (bind _controlledcharacter (`self.GetControlledCharacter` :!label _label)
        (:`OutPressed`
          (set `/Game/ExplosionsAndAction/Blueprints/Characters/BP_BaseCharacter.JumpButtonPressed` true _controlledcharacter))
        (:`OutReleased`
          (set `/Game/ExplosionsAndAction/Blueprints/Characters/BP_BaseCharacter.JumpButtonPressed` false _controlledcharacter)))
      (if (`/Game/ExplosionsAndAction/Blueprints/Characters/BP_BaseCharacter.InputEnabled` _controlledcharacter)
        (`/Game/ExplosionsAndAction/Blueprints/Characters/BP_BaseCharacter.MovementJump` _controlledcharacter AxisValue))
      (else
        ;[1 1 1] Handles Block input
        (set `self.JumpLast` false)
        (bind _controlledcharacter_2 (`self.GetControlledCharacter` :!label _label_2)
          (:`OutPressed`
            (if (`/Game/ExplosionsAndAction/Blueprints/Characters/BP_BaseCharacter.InputEnabled` _controlledcharacter_2)
              (`/Game/ExplosionsAndAction/Blueprints/Characters/BP_BaseCharacter.BlockPressed` _controlledcharacter_2)))
          (:`OutReleased`
            (`/Game/ExplosionsAndAction/Blueprints/Characters/BP_BaseCharacter.BlockReleased` _controlledcharacter_2)))))
    (elif (`self.JumpLast`)
      (goto _label :!via `Released`)
      (else
        (goto _label_2 :!via `Released`)))))

(event `requestServerRespawn`
  (params (`Class Type` :type "/Game/ExplosionsAndAction/Blueprints/Characters/CharacterTypes Enum" :default "NewEnumerator0"))
  (bind _returnvalue (`GameplayStatics.GetGameMode`))
  ;[1 1 1] Request Respawn
  (`/Engine/EditorBlueprintResources/ActorMacros.Switch Has Authority`
    (:`Authority`
      (`/Engine/EditorBlueprintResources/StandardMacros.IsValid` _returnvalue
        (:`Is Valid`
          (bind _asbase_game_mode (cast `/Game/ExplosionsAndAction/Blueprints/GameModes/BaseGameMode` _returnvalue))
          (`/Engine/EditorBlueprintResources/StandardMacros.IsValid` _asbase_game_mode
            (:`Is Valid`
              (bind _returnvalue_2 (`self.CastToPlayerController`))
              (`/Game/ExplosionsAndAction/Blueprints/GameModes/BaseGameMode.Respawn` _asbase_game_mode _returnvalue_2 `Class Type`))))))))

(event `InputAction|Fire`
  ;[1 1 1] Handles Fire Input
  (:`Pressed`
    (bind _controlledcharacter (`self.GetControlledCharacter` :!label _label_3)
      (:`OutPressed`
        (if (`/Game/ExplosionsAndAction/Blueprints/Characters/BP_BaseCharacter.InputEnabled` _controlledcharacter)
          (`/Game/ExplosionsAndAction/Blueprints/Characters/BP_BaseCharacter.EventWeaponFire` _controlledcharacter)))
      (:`OutReleased`
        (`/Game/ExplosionsAndAction/Blueprints/Characters/BP_BaseCharacter.EventStopWeaponFire` _controlledcharacter))))
  (:`Released`
    (goto _label_3 :!via `Released`)))

(event `KillMessage`
  (params (KilledBy :type String) (Killed :type String))
  ;[1 1 1] KillMessage
  (bind _asbase_game_instance (cast `/Game/ExplosionsAndAction/Blueprints/BaseGameInstance` (`GameplayStatics.GetGameInstance`)))
  (`/Game/ExplosionsAndAction/Blueprints/UI/HeadsUpDisplay.AddToKillLog` (`self.HUD`) (`KismetTextLibrary.Conv_StringToText` KilledBy) (`KismetTextLibrary.Conv_StringToText` Killed))
  (`/Game/ExplosionsAndAction/Blueprints/UI/HeadsUpDisplay.AddToKillLog` (`/Game/ExplosionsAndAction/Blueprints/BaseGameInstance.HUD` _asbase_game_instance) (`KismetTextLibrary.Conv_StringToText` KilledBy) (`KismetTextLibrary.Conv_StringToText` Killed)))

(event `InputAction|Fly`
  ;[1 1 1] Handles Fly Input
  (:`Pressed`
    (bind _controlledcharacter (`self.GetControlledCharacter` :!label _label_4)
      (:`OutPressed`
        (if (`/Game/ExplosionsAndAction/Blueprints/Characters/BP_BaseCharacter.InputEnabled` _controlledcharacter)
          (`/Game/ExplosionsAndAction/Blueprints/Characters/BP_BaseCharacter.EventStartFly` _controlledcharacter (`self.DeprojectMousePositionToWorld`))))
      (:`OutReleased`
        (`/Game/ExplosionsAndAction/Blueprints/Characters/BP_BaseCharacter.EventStopFly` _controlledcharacter))))
  (:`Released`
    (goto _label_4 :!via `Released`)))

(event `InputAction|Suicide`
  ;[1 1 1] Request Suicide
  (:`Pressed`
    (if (`self.IsLocalPlayerController`)
      (`/Engine/EditorBlueprintResources/StandardMacros.IsValid` (`self.K2_GetPawn`)
        (:`Is Valid`
          (`self.requestServerSuicide`))))))

(event `InputAction|Reload`
  ;[1 1 1] Handles Weapon Reload Input
  (:`Pressed`
    (bind _controlledcharacter (`self.GetControlledCharacter` :!label _label_5)
      (:`OutPressed`
        (if (`/Game/ExplosionsAndAction/Blueprints/Characters/BP_BaseCharacter.InputEnabled` _controlledcharacter)
          (`/Game/ExplosionsAndAction/Blueprints/Characters/BP_BaseCharacter.ReloadWeapon` _controlledcharacter)))))
  (:`Released`
    (goto _label_5 :!via `Released`)))

(event `requestServerSuicide`
  ;[1 1 1] Request Suicide
  (`GameplayStatics.ApplyDamage` (`self.K2_GetPawn`) 1000.0 null null "/Script/Engine.DamageType"))

(event `PrintMsg`
  (params (Message :type String))
  ;[1 1 1] PickupMessage
  (bind _asbase_game_instance (cast `/Game/ExplosionsAndAction/Blueprints/BaseGameInstance` (`GameplayStatics.GetGameInstance`)))
  (`/Game/ExplosionsAndAction/Blueprints/UI/HeadsUpDisplay.AddToPickUpLog` (`/Game/ExplosionsAndAction/Blueprints/BaseGameInstance.HUD` _asbase_game_instance) Message))

(event `InputAction|SwapWeapon`
  ;[1 1 1] Handles Weapon Swap Input
  (:`Pressed`
    (bind _controlledcharacter (`self.GetControlledCharacter` :!label _label_6)
      (:`OutPressed`
        (if (`/Game/ExplosionsAndAction/Blueprints/Characters/BP_BaseCharacter.InputEnabled` _controlledcharacter)
          (`/Game/ExplosionsAndAction/Blueprints/Characters/BP_BaseCharacter.WeaponSwap` _controlledcharacter)))))
  (:`Released`
    (goto _label_6 :!via `Released`)))

(event `InputAction|ScoreBoard`
  (bind _returnvalue (`GameplayStatics.GetGameInstance`))
  ;[1 1 1] ScoreBoard
  (:`Pressed`
    (bind _asbase_game_instance (cast `/Game/ExplosionsAndAction/Blueprints/BaseGameInstance` _returnvalue))
    (`/Game/ExplosionsAndAction/Blueprints/BaseGameInstance.ShowScoreBoard` _asbase_game_instance))
  (:`Released`
    (bind _asbase_game_instance_2 (cast `/Game/ExplosionsAndAction/Blueprints/BaseGameInstance` _returnvalue))
    (switch `/Game/ExplosionsAndAction/Blueprints/GameModes/GameModeStates` (`self.CurrentPlayingState`)
      (:`NewEnumerator0`
        (`/Game/ExplosionsAndAction/Blueprints/BaseGameInstance.ShowPlayingState` _asbase_game_instance_2))
      (:`NewEnumerator1`
        (`/Game/ExplosionsAndAction/Blueprints/BaseGameInstance.ShowSpawnMenu` _asbase_game_instance_2)))))

(event `ShowWinScreen`
  (params (WinningPlayer :type Text))
  ;[1 1 1] WinScreen
  (bind _asbase_game_instance (cast `/Game/ExplosionsAndAction/Blueprints/BaseGameInstance` (`GameplayStatics.GetGameInstance`)))
  (`/Game/ExplosionsAndAction/Blueprints/BaseGameInstance.ShowWinScreen` _asbase_game_instance WinningPlayer))

(fn `GetControlledIfInvalid`
  (`/Engine/EditorBlueprintResources/StandardMacros.IsValid` (`self.ControlledCharacter`)
    (:`Is Not Valid`
      (bind _asbp_base_character (cast `/Game/ExplosionsAndAction/Blueprints/Characters/BP_BaseCharacter` (`self.K2_GetPawn`)))
      (set `self.ControlledCharacter` _asbp_base_character))))

(fn `UserConstructionScript`)