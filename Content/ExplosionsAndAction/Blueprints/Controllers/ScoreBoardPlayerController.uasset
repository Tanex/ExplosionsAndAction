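; ScoreBoardPlayerController is a player controller that toggles the scoreboard while the ScoreBoard input action is held.
; Pressing the action casts the game instance to BaseGameInstance and calls ShowScoreBoard, and releasing it calls ShowPlayingState.
; The controller holds no other logic, so the game instance handles the actual display switching.
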(event `self.ReceiveBeginPlay`
  (`parent.ReceiveBeginPlay`))

(event `self.ReceiveTick`
  (params (DeltaSeconds :type "Float (single-precision)"))
  (`parent.ReceiveTick` 0.0))

(event `InputAction|ScoreBoard`
  (bind _returnvalue (`GameplayStatics.GetGameInstance`))
  (:`Pressed`
    (bind _asbase_game_instance (cast `/Game/ExplosionsAndAction/Blueprints/BaseGameInstance` _returnvalue))
    (`/Game/ExplosionsAndAction/Blueprints/BaseGameInstance.ShowScoreBoard` _asbase_game_instance))
  (:`Released`
    (bind _asbase_game_instance_2 (cast `/Game/ExplosionsAndAction/Blueprints/BaseGameInstance` _returnvalue))
    (`/Game/ExplosionsAndAction/Blueprints/BaseGameInstance.ShowPlayingState` _asbase_game_instance_2)))

(fn `UserConstructionScript`
  (`parent.UserConstructionScript`))