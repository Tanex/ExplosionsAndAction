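; Rocket projectile Blueprint that deals explosive area damage when its render component begins overlapping another actor.
; Overlaps with the instigator or actors tagged NoBulletCollide are ignored.
; Otherwise it applies radial damage with falloff at its location, credited to the instigator's controller, sparing all weapon actors and blockable by WorldStatic geometry.
; It then spawns the explosion emitter there; the graph does not destroy the rocket itself.
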(event `self.RenderComponent.OnComponentBeginOverlap`
  (params (OtherActor :type "Actor Object Reference") (OtherComp :type "PrimitiveComponent Object Reference") (OtherBodyIndex :type Integer) (bFromSweep :type Boolean) (SweepResult :type "EngineTypes.HitResult Structure (by ref)"))
  (bind _returnvalue (`self.K2_GetActorLocation`))
  (if (not (or (`self.ActorHasTag` OtherActor "NoBulletCollide") (== OtherActor (`self.GetInstigator`))))
    (bind _outactors (`GameplayStatics.GetAllActorsOfClass` "/Game/ExplosionsAndAction/Blueprints/Weapons/WeaponBaseClass.WeaponBaseClass_C"))
    (`GameplayStatics.ApplyRadialDamageWithFalloff` (`self.Damage`) 0.0 _returnvalue 100.0 500.0 2.0 "/Script/Engine.DamageType" _outactors self (`self.GetInstigatorController`) "ECC_WorldStatic")
    (`GameplayStatics.SpawnEmitterAtLocation` "/Game/ExplosionsAndAction/Particles/Explosion/Explosion.Explosion" _returnvalue)))

(fn `UserConstructionScript`
  (`parent.UserConstructionScript`))