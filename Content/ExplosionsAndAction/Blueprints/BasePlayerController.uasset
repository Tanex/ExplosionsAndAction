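; Base player controller for a side-view shooter, turning input and cursor position into actions on the possessed BP_BaseCharacter.
; Macros cache the character and forward movement, jump, fly, block, fire, reload and weapon-swap input.
; On local Tick, the deprojected mouse position flips control yaw left or right and rotates the weapon in the XZ plane.
; It also shows the GameInstance spawn menu, requests respawns through BaseGameMode, and handles suicide through lethal damage.
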(event `self.ReceiveBeginPlay`
  (`self.BindOnDestroyed`)
  (`self.ShowSpawnMenu`))

(event `BindOnDestroyed`
  (bind _returnvalue (`self.K2_GetPawn`))
  ;[1 1 1] Bind SpawnMenu to OnDestroyed
  (`/Engine/EditorBlueprintResources/StandardMacros.IsValid` _returnvalue
    (:`Is Valid`
      (add `self.OnDestroyed` _returnvalue (delegate `OnDestroyedEvent`)))))

(event `OnDestroyedEvent`
  ;[1 1 1] Show SpawnMenu when destroyed
  (`/Engine/EditorBlueprintResources/ActorMacros.Switch Has Authority`
    (:`Authority`
      (`self.ShowSpawnMenu`))))

(event `self.ReceiveTick`
  (params (DeltaSeconds :type "Float (single-precision)"))
  (bind _weaponsprite (`/Game/ExplosionsAndAction/Blueprints/Characters/BP_BaseCharacter.WeaponSprite` (`self.ControlledCharacter`)))
  ;[1 1 1] Handle Everything affected by cursor position
  (if (`self.IsLocalPlayerController`)
    (`self.GetControlledCharIfInvalid`
      (:`Out`
        (`self.GetMouseFlip`
          (:`FaceRight`
            (`self.SetControlRotation` (`KismetMathLibrary.MakeRot` 0.0 0.0))
            (`SceneComponent.K2_SetRelativeLocation` _weaponsprite (0.0 0.1 0.0) false))
          (:`FaceLeft`
            (`self.SetControlRotation` (`KismetMathLibrary.MakeRot` 0.0 180.0))
            (`SceneComponent.K2_SetRelativeLocation` _weaponsprite (0.0 -0.1 0.0) false))
          (:`Out`
            (bind _weaponrotation (`self.WeaponRotation`)
              (:`Out`
                (`/Game/ExplosionsAndAction/Blueprints/Characters/BP_BaseCharacter.RotateWeapon` (`self.ControlledCharacter`) _weaponrotation)))))))))

(event `InitSpawnMenu`
  ;[1 1 1] Show Spawn Menu
)

(event `ShowSpawnMenu`
  ;[1 1 1] Show Spawn Menu
  (bind _asbase_game_instance (cast `/Game/ExplosionsAndAction/Blueprints/BaseGameInstance` (`GameplayStatics.GetGameInstance`)))
  (`/Game/ExplosionsAndAction/Blueprints/BaseGameInstance.ShowSpawnMenu` _asbase_game_instance))

(event `InputAxis|MoveRight`
  (params (AxisValue :type "Float (single-precision)"))
  ;[1 1 1] Handles Horizontal Movement Input
  (`self.GetControlledCharIfInvalid`
    (:`Out`
      (`/Game/ExplosionsAndAction/Blueprints/Characters/BP_BaseCharacter.MovementHorizontal` (`self.ControlledCharacter`) AxisValue))))

(event `InputAction|Jump`
  ;[1 1 1] Handles Jump Input
  (:`Pressed`
    (bind _controlledcharacter (`self.GetControlledCharacter` :!label _label)
      (:`OutPressed`
        (set `/Game/ExplosionsAndAction/Blueprints/Characters/BP_BaseCharacter.JumpButtonPressed` true _controlledcharacter))
      (:`OutReleased`
        (set `/Game/ExplosionsAndAction/Blueprints/Characters/BP_BaseCharacter.JumpButtonPressed` false _controlledcharacter)))
    (`/Game/ExplosionsAndAction/Blueprints/Characters/BP_BaseCharacter.MovementJump` _controlledcharacter))
  (:`Released`
    (goto _label :!via `Released`)))

(event `EventRequestRespawn`
  ;[1 1 1] Request Respawn
  (if (`self.IsLocalPlayerController`)
    (`/Engine/EditorBlueprintResources/StandardMacros.IsValid` (`self.K2_GetPawn`)
      (:`Is Not Valid`
        (`self.requestServerRespawn`)))))

(event `InputAction|Fire`
  ;[1 1 1] Handles Fire Input
  (:`Pressed`
    (bind _controlledcharacter (`self.GetControlledCharacter` :!label _label_2)
      (:`OutPressed`
        (`/Game/ExplosionsAndAction/Blueprints/Characters/BP_BaseCharacter.EventWeaponFire` _controlledcharacter))
      (:`OutReleased`
        (`/Game/ExplosionsAndAction/Blueprints/Characters/BP_BaseCharacter.EventStopWeaponFire` _controlledcharacter))))
  (:`Released`
    (goto _label_2 :!via `Released`)))

(event `requestServerRespawn`
  (bind _returnvalue (`GameplayStatics.GetGameMode`))
  ;[1 1 1] Request Respawn
  (`/Engine/EditorBlueprintResources/ActorMacros.Switch Has Authority`
    (:`Authority`
      (`/Engine/EditorBlueprintResources/StandardMacros.IsValid` _returnvalue
        (:`Is Valid`
          (bind _asbase_game_mode (cast `/Game/ExplosionsAndAction/Blueprints/GameModes/BaseGameMode` _returnvalue))
          (`/Engine/EditorBlueprintResources/StandardMacros.IsValid` _asbase_game_mode
            (:`Is Valid`
              (bind _returnvalue_2 (`self.CastToPlayerController`))
              (`/Game/ExplosionsAndAction/Blueprints/GameModes/BaseGameMode.Respawn` _asbase_game_mode _returnvalue_2))))))))

(event `InputAction|Fly`
  ;[1 1 1] Handles Fly Input
  (:`Pressed`
    (bind _controlledcharacter (`self.GetControlledCharacter` :!label _label_3)
      (:`OutPressed`
        (`/Game/ExplosionsAndAction/Blueprints/Characters/BP_BaseCharacter.EventStartFly` _controlledcharacter))
      (:`OutReleased`
        (`/Game/ExplosionsAndAction/Blueprints/Characters/BP_BaseCharacter.EventStopFly` _controlledcharacter))))
  (:`Released`
    (goto _label_3 :!via `Released`)))

(event `InputAction|Block`
  ;[1 1 1] Handles Block input
  (:`Pressed`
    (bind _controlledcharacter (`self.GetControlledCharacter` :!label _label_4)
      (:`OutPressed`
        (set `/Game/ExplosionsAndAction/Blueprints/Characters/BP_BaseCharacter.BlockButtonPressed` true _controlledcharacter))
      (:`OutReleased`
        (set `/Game/ExplosionsAndAction/Blueprints/Characters/BP_BaseCharacter.BlockButtonPressed` false _controlledcharacter)))
    (`/Game/ExplosionsAndAction/Blueprints/Characters/BP_BaseCharacter.MovementBlock` _controlledcharacter))
  (:`Released`
    (goto _label_4 :!via `Released`)))

(event `InputAction|Suicide`
  ;[1 1 1] Request Suicide
  (:`Pressed`
    (if (`self.IsLocalPlayerController`)
      (`/Engine/EditorBlueprintResources/StandardMacros.IsValid` (`self.K2_GetPawn`)
        (:`Is Valid`
          (`self.requestServerSuicide`))))))

(event `InputAction|Reload`
  ;[1 1 1] Handles Weapon Reload Input
  (:`Pressed`
    (bind _controlledcharacter (`self.GetControlledCharacter` :!label _label_5)
      (:`OutPressed`
        (set `/Game/ExplosionsAndAction/Blueprints/Characters/BP_BaseCharacter.ReloadButtonPressed` true _controlledcharacter))
      (:`OutReleased`
        (set `/Game/ExplosionsAndAction/Blueprints/Characters/BP_BaseCharacter.ReloadButtonPressed` false _controlledcharacter)))
    (`/Game/ExplosionsAndAction/Blueprints/Characters/BP_BaseCharacter.WeaponReload` _controlledcharacter))
  (:`Released`
    (goto _label_5 :!via `Released`)))

(event `requestServerSuicide`
  ;[1 1 1] Request Suicide
  (`GameplayStatics.ApplyDamage` (`self.K2_GetPawn`) 1000.0 null null "/Script/Engine.DamageType"))

(event `InputAction|SwapWeapon`
  ;[1 1 1] Handles Weapon Swap Input
  (:`Pressed`
    (bind _controlledcharacter (`self.GetControlledCharacter` :!label _label_6)
      (:`OutPressed`
        (set `/Game/ExplosionsAndAction/Blueprints/Characters/BP_BaseCharacter.SwapButtonPressed` false _controlledcharacter))
      (:`OutReleased`
        (set `/Game/ExplosionsAndAction/Blueprints/Characters/BP_BaseCharacter.SwapButtonPressed` false _controlledcharacter)))
    (`/Game/ExplosionsAndAction/Blueprints/Characters/BP_BaseCharacter.WeaponSwap` _controlledcharacter))
  (:`Released`
    (goto _label_6 :!via `Released`)))

(fn `GetControlledIfInvalid`
  (`/Engine/EditorBlueprintResources/StandardMacros.IsValid` (`self.ControlledCharacter`)
    (:`Is Not Valid`
      (bind _asbp_base_character (cast `/Game/ExplosionsAndAction/Blueprints/Characters/BP_BaseCharacter` (`self.K2_GetPawn`)))
      (set `self.ControlledCharacter` _asbp_base_character))))

(fn `UserConstructionScript`)