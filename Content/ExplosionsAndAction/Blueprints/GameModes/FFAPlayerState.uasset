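; Player state for the free-for-all mode that holds a player's score and per-pickup, class and weapon statistics.
; UpdateScore increments and prints PlayerScore, whose RepNotify has the server ask FFAGameMode to CheckWin.
; The stat updaters find an entry by ID and accumulate into it, or append one, using a shared StatsFound flag.
; Updating an existing pickup entry resets its kill count to zero instead of adding.
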(event `self.ReceiveBeginPlay`)

(event `self.ReceiveTick`
  (params (DeltaSeconds :type "Float (single-precision)")))

(fn `OnRep_PlayerScore`
  (`/Engine/EditorBlueprintResources/ActorMacros.Switch Has Authority`
    (:`Authority`
      (bind _asffagame_mode (cast `/Game/ExplosionsAndAction/Blueprints/GameModes/FFAGameMode` (`GameplayStatics.GetGameMode`))
        (:`then`
          (`/Game/ExplosionsAndAction/Blueprints/GameModes/FFAGameMode.CheckWin` _asffagame_mode))
        (:`CastFailed`
          (`KismetSystemLibrary.PrintString` "Hello"))))))

(fn `UpdateClassStats`
  (params (ClassId :type Integer :default 0) (DamageTaken :type Integer :default 0) (NumDeaths :type Integer :default 0))
  (for (_array_element _array_index) (`self.ClassStats`)
    (bind (_classid _damagetaken _numdeaths) (break `/Game/ExplosionsAndAction/Blueprints/Logging/ClassStats` _array_element))
    (if (== _classid ClassId)
      (`KismetArrayLibrary.Array_Set` (`self.ClassStats`) _array_index (make `/Game/ExplosionsAndAction/Blueprints/Logging/ClassStats` _classid (+ _damagetaken DamageTaken) (+ _numdeaths NumDeaths)))
      (set `self.StatsFound` true)
      (break)))
  (if (not (`self.StatsFound`))
    (`KismetArrayLibrary.Array_Add` (`self.ClassStats`) (make `/Game/ExplosionsAndAction/Blueprints/Logging/ClassStats` ClassId DamageTaken NumDeaths)))
  (set `self.StatsFound` false))

(fn `UpdatePickupStats`
  (params (pickupId :type Integer :default 0) (taken :type Integer :default 0) (kill :type Integer :default 0))
  (for (_array_element _array_index) (`self.PickupStats`)
    (bind (_pickupid _numtaken) (break `/Game/ExplosionsAndAction/Blueprints/Logging/PickupStats` _array_element))
    (if (== _pickupid pickupId)
      (`KismetArrayLibrary.Array_Set` (`self.PickupStats`) _array_index (make `/Game/ExplosionsAndAction/Blueprints/Logging/PickupStats` _pickupid (+ _numtaken taken)))
      (set `self.StatsFound` true)
      (break)))
  (if (not (`self.StatsFound`))
    (`KismetArrayLibrary.Array_Add` (`self.PickupStats`) (make `/Game/ExplosionsAndAction/Blueprints/Logging/PickupStats` pickupId taken kill)))
  (set `self.StatsFound` false))

(fn `UpdateScore`
  (params (`Increment By` :type Integer :default 0))
  (bind _playerscore (`self.PlayerScore`))
  (set `self.PlayerScore` (+ _playerscore `Increment By`))
  (`KismetSystemLibrary.PrintString` (`KismetStringLibrary.Conv_IntToString` _playerscore)))

(fn `UpdateWeaponStats`
  (params (WeaponId :type Integer :default 0) (NumKills :type Integer :default 0) (NumHits :type Integer :default 0) (ShotsFired :type Integer :default 0) (DamageAmount :type Integer :default 0))
  (for (_array_element _array_index) (`self.WeaponStats`)
    (bind (_weaponid _numkills _numhits _shotsfired _damageamount) (break `/Game/ExplosionsAndAction/Blueprints/Logging/WeaponStats` _array_element))
    (if (== _weaponid WeaponId)
      (`KismetArrayLibrary.Array_Set` (`self.WeaponStats`) _array_index (make `/Game/ExplosionsAndAction/Blueprints/Logging/WeaponStats` _weaponid (+ _numkills NumKills) (+ _numhits NumHits) (+ _shotsfired ShotsFired) (+ _damageamount DamageAmount)))
      (set `self.StatsFound` true)
      (break)))
  (if (not (`self.StatsFound`))
    (`KismetArrayLibrary.Array_Add` (`self.WeaponStats`) (make `/Game/ExplosionsAndAction/Blueprints/Logging/WeaponStats` WeaponId NumKills NumHits ShotsFired DamageAmount)))
  (set `self.StatsFound` false))

(fn `UserConstructionScript`)