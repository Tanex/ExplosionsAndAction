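; Free-for-all game mode that handles soldier respawns and ends a match at the frag limit.
; On BeginPlay the server caches all PlayerStarts, and Respawn spawns a BP_SoldierCharacter at a random one for the controller to possess.
; CheckWin scans player controllers by index and reopens "Map" via OpenLevel when any FFAPlayerState score reaches FragLimit.
; A servertravel command is left unconnected.
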(event `CheckWin`
  ;[1 1 1] Check for winners
  (for _index (range 33)
    (bind _returnvalue (`GameplayStatics.GetPlayerController` _index))
    (`/Engine/EditorBlueprintResources/StandardMacros.IsValid` _returnvalue
      (:`Is Valid`
        (bind _asffaplayer_state (cast `/Game/ExplosionsAndAction/Blueprints/GameModes/FFAPlayerState` (`Controller.PlayerState` _returnvalue)))
        (if (>= (`/Game/ExplosionsAndAction/Blueprints/GameModes/FFAPlayerState.PlayerScore` _asffaplayer_state) (`self.FragLimit`))
          (`GameplayStatics.OpenLevel` "Map"))))))

(event `self.ReceiveBeginPlay`
  ;[1 1 1] Set array of all spawnpoints
  (`parent.ReceiveBeginPlay`)
  (`/Engine/EditorBlueprintResources/ActorMacros.Switch Has Authority`
    (:`Authority`
      (`KismetArrayLibrary.Array_Clear` (`self.PlayerStart`))
      (bind _outactors (`GameplayStatics.GetAllActorsOfClass` "/Script/Engine.PlayerStart"))
      (set `self.PlayerStart` _outactors))))

(event `Respawn`
  (params (`Player Controller` :type "PlayerController Object Reference"))
  (bind _playerstart (`self.PlayerStart`))
  ;[1 1 1] Respawn
  (`/Engine/EditorBlueprintResources/StandardMacros.IsValid` `Player Controller`
    (:`Is Valid`
      (`/Engine/EditorBlueprintResources/ActorMacros.Switch Has Authority`
        (:`Authority`
          (bind _returnvalue (`|SpawnActorFromClass` "/Game/ExplosionsAndAction/Blueprints/Characters/BP_SoldierCharacter.BP_SoldierCharacter_C" (`self.GetTransform` (`KismetArrayLibrary.Array_Get` _playerstart (`KismetMathLibrary.RandomIntegerInRange` 0 (- (`KismetArrayLibrary.Array_Length` _playerstart) 1))))))
          (`/Engine/EditorBlueprintResources/StandardMacros.IsValid` _returnvalue
            (:`Is Valid`
              (`Controller.Possess` `Player Controller` _returnvalue))))))))

(fn `UserConstructionScript`
  (`parent.UserConstructionScript`))