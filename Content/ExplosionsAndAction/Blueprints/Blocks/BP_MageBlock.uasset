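; Mage block shield attached to a BP_BaseCharacter that soaks damage and fires projectiles back.
; Construction sets its hit point pool, recharge tuning and collision response on the render component.
; Damage updates the owner's shield hit points and drains the pool; on depletion the block disables itself, passing any excess damage to the owner.
; While it holds, AmmoBaseClass hits are reflected by spawning the same class ahead of the owner's Block component.
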(event `self.ReceiveBeginPlay`)

(event `self.ReceiveActorBeginOverlap`
  (params (OtherActor :type "Actor Object Reference")))

(event `self.ReceiveTick`
  (params (DeltaSeconds :type "Float (single-precision)"))
  (`parent.ReceiveTick` 0.0))

(event `self.ReceiveAnyDamage`
  (params (Damage :type "Float (single-precision)") (DamageType :type "DamageType Object Reference") (InstigatedBy :type "Controller Object Reference") (DamageCauser :type "Actor Object Reference"))
  (bind _returnvalue (`ActorComponent.GetOwner` (`SceneComponent.GetAttachParent` (`self.K2_GetRootComponent`))))
  (bind _asbp_base_character (cast `/Game/ExplosionsAndAction/Blueprints/Characters/BP_BaseCharacter` _returnvalue))
  (`/Game/ExplosionsAndAction/Blueprints/Characters/BP_BaseCharacter.UpdateShieldHitPoints` _asbp_base_character 0.0)
  (bind _output_get (set `self.HitPoints` (- (`self.HitPoints`) Damage)))
  (if (<= _output_get 0.0)
    (if (< (`self.HitPoints`) 0.0)
      (`GameplayStatics.ApplyDamage` _returnvalue (`KismetMathLibrary.Abs` (`self.HitPoints`)) InstigatedBy DamageCauser "/Script/Engine.DamageType")
      (set `self.HitPoints` 0.0))
    (set `self.WasDestroyed` true)
    (set `self.CanBeActivated` false)
    (`self.SetEnable` false)
    (else
      (bind _asbp_base_character_2 (cast `/Game/ExplosionsAndAction/Blueprints/Characters/BP_BaseCharacter` (`ActorComponent.GetOwner` (`SceneComponent.GetAttachParent` (`self.K2_GetRootComponent`)))))
      (bind _asammo_base_class (cast `/Game/ExplosionsAndAction/Blueprints/Ammo/AmmoBaseClass` DamageCauser))
      (bind _asactor (castclass `Actor` (`GameplayStatics.GetObjectClass` _asammo_base_class)))
      (bind _block (`/Game/ExplosionsAndAction/Blueprints/Characters/BP_BaseCharacter.Block` _asbp_base_character_2))
      (`|SpawnActorFromClass` _asactor (`KismetMathLibrary.MakeTransform` (+ (`SceneComponent.K2_GetComponentLocation` _block) (* (`SceneComponent.GetForwardVector` _block) 200.0)) (`SceneComponent.K2_GetComponentRotation` _block) (`self.GetActorScale3D`)) false _asbp_base_character_2))))

(fn `UserConstructionScript`
  (bind _rendercomponent (`self.RenderComponent`))
  (`parent.UserConstructionScript`)
  (bind _output_get (set `self.MaxHitPoints` 75.0))
  (set `self.HitPoints` _output_get)
  (set `self.TickTriggerDelay` 0.5)
  (set `self.RechargeRate` 5.0)
  (`PrimitiveComponent.SetCollisionObjectType` _rendercomponent "ECC_WorldDynamic")
  (`PrimitiveComponent.SetCollisionResponseToChannel` _rendercomponent "ECC_GameTraceChannel1" "ECR_Overlap"))