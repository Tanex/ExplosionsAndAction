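; SHiddoshsh is a block Blueprint with unfinished, unreachable logic for spawning ammo from the character it is attached to.
; The disconnected chain finds the owning BP_BaseCharacter through the root's attach parent and would spawn an ammo-derived class ahead of its Block component, with that character as instigator.
; No event triggers it, the ammo cast has no input, and the construction script is empty.
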(fn `UserConstructionScript`)