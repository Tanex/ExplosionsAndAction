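; BP_MeleeBlock is a block attached to another actor that deals melee damage to characters it hits.
; When its RenderComponent registers a hit, it ignores the owner of the component it is attached to and only accepts BP_BaseCharacter targets.
; It applies BlockDamage to the target, crediting the attach parent owner's instigator controller, with itself as the damage causer.
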(event `self.ReceiveBeginPlay`)

(event `self.RenderComponent.OnComponentHit`
  (params (OtherActor :type "Actor Object Reference") (OtherComp :type "PrimitiveComponent Object Reference") (NormalImpulse :type "Object.Vector Structure") (Hit :type "EngineTypes.HitResult Structure (by ref)"))
  (bind _returnvalue (`ActorComponent.GetOwner` (`SceneComponent.GetAttachParent` (`self.K2_GetRootComponent`))))
  (if (!= _returnvalue OtherActor)
    (bind _asbp_base_character (cast `/Game/ExplosionsAndAction/Blueprints/Characters/BP_BaseCharacter` OtherActor))
    (`GameplayStatics.ApplyDamage` _asbp_base_character (`self.BlockDamage`) (`self.GetInstigatorController` _returnvalue) self "/Script/Engine.DamageType")))

(event `self.ReceiveTick`
  (params (DeltaSeconds :type "Float (single-precision)"))
  (`parent.ReceiveTick` 0.0))

(fn `UserConstructionScript`
  (`parent.UserConstructionScript`))