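; BP_CyborgBlock is a destructible block variant that damages itself whenever its IsVisibleTick event fires.
; Each firing applies a small fixed amount of damage through ApplyDamage, reduced to the remaining HitPoints when fewer are left.
; The construction script calls the parent's, then sets maximum and current hit points, the tick trigger delay and the recharge rate, none of which the child's graphs use except HitPoints.
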(event `self.ReceiveBeginPlay`)

(event `self.ReceiveActorBeginOverlap`
  (params (OtherActor :type "Actor Object Reference")))

(event `self.ReceiveTick`
  (params (DeltaSeconds :type "Float (single-precision)"))
  (`parent.ReceiveTick` 0.0))

(event `self.IsVisibleTick`
  (bind _hitpoints (`self.HitPoints`))
  (if (< _hitpoints 3.0)
    (`GameplayStatics.ApplyDamage` self _hitpoints null null "/Script/Engine.DamageType")
    (else
      (`GameplayStatics.ApplyDamage` self 3.0 null null "/Script/Engine.DamageType"))))

(fn `UserConstructionScript`
  (`parent.UserConstructionScript`)
  (bind _output_get (set `self.MaxHitPoints` 50.0))
  (set `self.HitPoints` _output_get)
  (set `self.TickTriggerDelay` 0.5)
  (set `self.RechargeRate` 2.0))