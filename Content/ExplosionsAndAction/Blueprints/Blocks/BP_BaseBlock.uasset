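; Base shield block attached to a BP_BaseCharacter, toggled by press and release to absorb damage.
; Toggling switches visibility, collision and damageability, with a cooldown after release.
; Damage drains hit points; at zero the shield disables until fully recharged, passing any excess damage to the owner.
; A delay-throttled, server-authoritative Tick recharges it while hidden, reporting hit points to the owning character.
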(event `Update`
  (`/Engine/EditorBlueprintResources/ActorMacros.Switch Has Authority`
    (:`Authority`
      (bind _asbp_base_character (cast `/Game/ExplosionsAndAction/Blueprints/Characters/BP_BaseCharacter` (`ActorComponent.GetOwner` (`SceneComponent.GetAttachParent` (`self.K2_GetRootComponent`)))))
      (`/Game/ExplosionsAndAction/Blueprints/Characters/BP_BaseCharacter.UpdateShieldHitPoints` _asbp_base_character (`self.HitPoints`)))))

(event `self.ReceiveBeginPlay`
  (`self.Update`))

(event `SetEnable`
  (params (Enable :type Boolean :default false))
  (if (`KismetSystemLibrary.IsValid` (`self.RenderComponent`))
    (set `self.Enabled` Enable)
    (set `PrimitiveComponent.bGenerateOverlapEvents` Enable (`self.RenderComponent`))
    (`self.SetActorEnableCollision` Enable)
    (`self.SetActorHiddenInGame` (not Enable))
    (set `self.bCanBeDamaged` Enable)
    (if Enable
      (`PrimitiveComponent.SetCollisionResponseToChannel` "ECC_Visibility" "ECR_Block")
      (else
        (`PrimitiveComponent.SetCollisionResponseToChannel` "ECC_Visibility" "ECR_Ignore")))))

(event `BlockPressed`
  ;[1 1 1] Activate Block
  (if (and (`self.CanBeActivated`) (not (`self.Enabled`)))
    (`self.SetEnable` true)
    (bind _asbp_base_character (cast `/Game/ExplosionsAndAction/Blueprints/Characters/BP_BaseCharacter` (`ActorComponent.GetOwner` (`SceneComponent.GetAttachParent` (`self.K2_GetRootComponent`)))))
    (`/Game/ExplosionsAndAction/Blueprints/Characters/BP_BaseCharacter.PlaySound` _asbp_base_character "/Game/ExplosionsAndAction/Sounds/Soldier_Riot_Shield_Equip.Soldier_Riot_Shield_Equip")))

(event `BlockReleased`
  ;[1 1 1] Deactivate Block
  (if (and (`self.CanBeActivated`) (not (`self.bHidden`)) (`self.Enabled`))
    (set `self.CanBeActivated` false)
    (`self.SetEnable` false)
    (if (not (`self.WasDestroyed`))
      (`KismetSystemLibrary.Delay` (`self.DeactivateCD`))
      (set `self.CanBeActivated` true))))

(event `self.ReceiveAnyDamage`
  (params (Damage :type "Float (single-precision)") (DamageType :type "DamageType Object Reference") (InstigatedBy :type "Controller Object Reference") (DamageCauser :type "Actor Object Reference"))
  (bind _returnvalue (`ActorComponent.GetOwner` (`SceneComponent.GetAttachParent` (`self.K2_GetRootComponent`))))
  ;[1 1 1] Take Damage, propagate to owner if dead
  (bind _asbp_base_character (cast `/Game/ExplosionsAndAction/Blueprints/Characters/BP_BaseCharacter` _returnvalue))
  (`/Game/ExplosionsAndAction/Blueprints/Characters/BP_BaseCharacter.UpdateShieldHitPoints` _asbp_base_character (`self.HitPoints`))
  (bind _output_get (set `self.HitPoints` (- (`self.HitPoints`) Damage)))
  (if (<= _output_get 0.0)
    (if (< (`self.HitPoints`) 0.0)
      (`GameplayStatics.ApplyDamage` _returnvalue (`KismetMathLibrary.Abs` (`self.HitPoints`)) InstigatedBy DamageCauser "/Script/Engine.DamageType")
      (set `self.HitPoints` 0.0))
    (set `self.WasDestroyed` true)
    (set `self.CanBeActivated` false)
    (`self.SetEnable` false)))

(event `self.ReceiveTick`
  (params (DeltaSeconds :type "Float (single-precision)"))
  ;[1 1 1] Event Tick
  (`/Engine/EditorBlueprintResources/ActorMacros.Switch Has Authority`
    (:`Authority`
      (`KismetSystemLibrary.Delay` (`self.TickTriggerDelay`))
      (if (`self.bHidden`)
        (`self.NotVisibleTick`)
        (else
          (`self.IsVisibleTick`))))))

(fn `IsVisibleTick`)

(fn `NotVisibleTick`
  (bind _maxhitpoints (`self.MaxHitPoints`))
  (if (< (`self.HitPoints`) (`self.MaxHitPoints`))
    (bind _output_get (set `self.HitPoints` (+ (`self.HitPoints`) (`self.RechargeRate`))))
    (`self.Update`)
    (if (>= (`self.HitPoints`) _maxhitpoints)
      (set `self.HitPoints` _maxhitpoints)
      (cast `/Game/ExplosionsAndAction/Blueprints/Characters/BP_BaseCharacter` (`ActorComponent.GetOwner` (`SceneComponent.GetAttachParent` (`self.K2_GetRootComponent`))))
      (if (`self.WasDestroyed`)
        (set `self.WasDestroyed` false)
        (set `self.CanBeActivated` true)))))

(fn `UserConstructionScript`
  (`SceneComponent.SetRelativeScale3D` (0.289855 0.289855 0.289855))
  (set `self.HitPoints` (`self.MaxHitPoints`))
  (set `self.WasDestroyed` false)
  (set `self.CanBeActivated` true)
  (`self.SetEnable` false))