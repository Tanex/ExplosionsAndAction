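; BP_Bullet is a bullet actor that damages what it overlaps.
; On overlap it skips its instigator and actors tagged NoBulletCollide, otherwise applies damage, disables overlaps, hides itself and shortens its lifespan for delayed destruction.
; The construction script sets a fallback lifespan for stray bullets and doubles damage if the instigating BP_BaseCharacter's PickupHandler has double damage.
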(event `self.RenderComponent.OnComponentBeginOverlap`
  (params (OtherActor :type "Actor Object Reference") (OtherComp :type "PrimitiveComponent Object Reference") (OtherBodyIndex :type Integer) (bFromSweep :type Boolean) (SweepResult :type "EngineTypes.HitResult Structure (by ref)"))
  ;[1 1 1] Do damage on hit
  (if (not (or (`self.ActorHasTag` OtherActor "NoBulletCollide") (== OtherActor (`self.GetInstigator`))))
    (`GameplayStatics.ApplyDamage` OtherActor (`self.BulletDamage`) (`self.GetInstigatorController`) self "/Script/Engine.DamageType")
    (set `PrimitiveComponent.bGenerateOverlapEvents` false (`self.RenderComponent`))
    (`self.SetActorHiddenInGame` true)
    (`self.SetLifeSpan` 2.0)))

(fn `UserConstructionScript`
  ;[1 1 1] Make sure stray bullets are destroyed
  (`self.SetLifeSpan` 10.0)
  ;[1 1 1] Check double damage
  (bind _asbp_base_character (cast `/Game/ExplosionsAndAction/Blueprints/Characters/BP_BaseCharacter` (`self.GetInstigator`)))
  (if (`/Game/ExplosionsAndAction/Blueprints/Characters/PickupHandler.HasDoubleDamage` (`/Game/ExplosionsAndAction/Blueprints/Characters/BP_BaseCharacter.PickupHandler` _asbp_base_character))
    (set `self.BulletDamage` (* (`self.BulletDamage`) 2.0))))